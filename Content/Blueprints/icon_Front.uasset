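; Front icon actor that shows a material billboard marker coloured by type: friendly, enemy or unknown.
; The construction script creates a dynamic material instance, then sets its icon texture and colour and rebuilds the sprite at a given size, optionally flipped vertically by negating its height.
; Tick pushes the Opacity value into the material's fade parameter every frame.
; A helper function hides or shows the billboard in game.
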(event `self.ReceiveTick`
  (params (DeltaSeconds :type "Float (single-precision)"))
  (`MaterialInstanceDynamic.SetScalarParameterValue` (`self.dynamat`) "Opacity Fade" (`self.Opacity`)))

(fn `Change_Icon_Elements`
  (params (Size :type "Float (double-precision)"))
  (bind _dynamat (`self.dynamat`))
  (bind _size (`self.size`))
  (set `self.size` Size)
  (`MaterialInstanceDynamic.SetTextureParameterValue` _dynamat "Icon" (`self.Side Icon`))
  (`MaterialInstanceDynamic.SetVectorParameterValue` _dynamat "Colour" (select `/Game/Blueprints/Enums/Icon_Type` (`self.icon type`) :`NewEnumerator0` (`self.Friendly`) :`NewEnumerator1` (`self.Enemy`) :`NewEnumerator2` (`self.Unknown`)))
  (`MaterialBillboardComponent.SetElements` (`self.MaterialBillboard`) (`|MakeArray` (make `MaterialSpriteElement` (`self.dynamat`) null false _size (select `bool` (`self.flipped`) :`false` _size :`true` (* _size -1.0))))))

(fn `hide_Icon`
  (params (NewHidden :type Boolean))
  (`SceneComponent.SetHiddenInGame` (`self.MaterialBillboard`) NewHidden false))

(fn `UserConstructionScript`
  (bind _returnvalue (`PrimitiveComponent.CreateDynamicMaterialInstance` (`self.MaterialBillboard`) 0 "/Game/_CEARepositoryFiles/2DAssets/Icons/Basic/Icon_Front_MatInst.Icon_Front_MatInst" "None"))
  (set `self.dynamat` _returnvalue)
  (`self.Change_Icon_Elements` (`self.size`))
  (`MaterialInstanceDynamic.SetScalarParameterValue` (`self.dynamat`) "Opacity Fade" (`self.Opacity`)))