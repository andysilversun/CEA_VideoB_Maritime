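; Child actor of Decal_actor that displays a coloured band letter (X, C, S or L) as a billboard.
; Construction creates a dynamic material, and UpdateLetter sets its texture and colour, rebuilding the sprite at the given size.
; Each Tick traces vertically, ignoring the parent decal, and hides the billboard if the first hit is another Decal_actor.
; Otherwise it shows the letter and moves it above the impact point by the parent's LetterHeight.
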(event `self.ReceiveTick`
  (params (DeltaSeconds :type "Float (single-precision)"))
  (bind _materialbillboard (`self.MaterialBillboard`))
  (bind (_returnvalue_x _returnvalue_y _returnvalue_z) (`KismetMathLibrary.BreakVector` (`SceneComponent.K2_GetComponentLocation` (`self.Arrow`))))
  (bind _returnvalue (+ _returnvalue_z 100000.0))
  (bind _outhits (`KismetSystemLibrary.LineTraceMultiForObjects` (`KismetMathLibrary.MakeVector` _returnvalue_x _returnvalue_y _returnvalue) (`KismetMathLibrary.MakeVector` _returnvalue_x _returnvalue_y (* _returnvalue -1.0)) (`|MakeArray` "ObjectTypeQuery1" "ObjectTypeQuery2" :!type "EObjectTypeQuery Enum") false (`|MakeArray` (`self.decal_Parent`))))
  (for _array_element _outhits
    (bind (_bblockinghit _binitialoverlap _time _distance _location _impactpoint _normal _impactnormal _physmat _hitactor) (`GameplayStatics.BreakHitResult` _array_element))
    (cast `/Game/Blueprints/Decal_actor` _hitactor
      (:`then`
        (`SceneComponent.SetVisibility` _materialbillboard false false)
        (break))
      (:`CastFailed`
        (bind _asdecal_actor (cast `/Game/Blueprints/Decal_actor` (`self.GetParentActor`)))
        (`self.K2_SetActorLocation` (+ _impactpoint (* (`KismetMathLibrary.GetUpVector` (struct)) (* (`/Game/Blueprints/Decal_actor.Letter_Height` _asdecal_actor) 100.0))) true)
        (`SceneComponent.SetVisibility` _materialbillboard true false)
        (break)))))

(event `UpdateLetter`
  (params (newLetter :type "/Game/Blueprints/Enums/BandLetters Enum" :default "NewEnumerator0") (newParent :type "Actor Object Reference") (newColour :type "LinearColor Structure") (initialSize :type "Float (double-precision)"))
  (bind _returnvalue (/ initialSize 100.0))
  (bind _billboard (`self.Billboard`))
  (bind (_material _distancetoopacitycurve _bsizeisinscreenspace _basesizex _basesizey _distancetosizecurve) (break `MaterialSpriteElement` (`|GetArrayItem` (`MaterialBillboardComponent.Elements` (`self.MaterialBillboard`)))))
  (bind _output_get (set `self.Band Letters` newLetter))
  (set `self.decal_Parent` newParent)
  (`MaterialInstanceDynamic.SetTextureParameterValue` _billboard "Letter" (select `/Game/Blueprints/Enums/BandLetters` _output_get :`NewEnumerator0` "/Game/_CEARepositoryFiles/2DAssets/Icons/Radar/X.X" :`NewEnumerator2` "/Game/_CEARepositoryFiles/2DAssets/Icons/Radar/C.C" :`NewEnumerator1` "/Game/_CEARepositoryFiles/2DAssets/Icons/Radar/S.S" :`NewEnumerator3` "/Game/_CEARepositoryFiles/2DAssets/Icons/Radar/L.L" :!type "Texture2D Object Reference"))
  (`MaterialInstanceDynamic.SetVectorParameterValue` _billboard "Colour" newColour)
  (`MaterialBillboardComponent.SetElements` (`self.MaterialBillboard`) (`|MakeArray` (make `MaterialSpriteElement` _billboard _distancetoopacitycurve _bsizeisinscreenspace _returnvalue _returnvalue _distancetosizecurve))))

(fn `hide_letter`
  (params (NewHidden :type Boolean))
  (`SceneComponent.SetHiddenInGame` (`self.MaterialBillboard`) NewHidden false))

(fn `UserConstructionScript`
  (bind _billboard (`self.Billboard`))
  (bind _returnvalue (`PrimitiveComponent.CreateDynamicMaterialInstance` (`self.MaterialBillboard`) 0 null "None"))
  (set `self.Billboard` _returnvalue)
  (`MaterialInstanceDynamic.SetTextureParameterValue` _billboard "Letter" (select `/Game/Blueprints/Enums/BandLetters` (`self.Band Letters`) :!type "Texture2D Object Reference"))
  (`MaterialInstanceDynamic.SetVectorParameterValue` _billboard "Colour" (`self.Colour`)))