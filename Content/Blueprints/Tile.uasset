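; Radar tile actor that displays a centred grid of 8x8 radar meshes and/or an X/C/S/L band overlay.
; SelfState, set locally, by a vehicle or from the game instance's global state, selects hidden, detailed, public (LOD) or band-only display.
; Detailed and public states add instanced meshes by row and column count, optionally overlaying a scaled, band-coloured box and letter.
; Setup runs at construction and when Tick sees the Update flag.
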(event `self.ReceiveBeginPlay`)

(event `self.ReceiveTick`
  (params (DeltaSeconds :type "Float (single-precision)"))
  (if (`self.Update`)
    (`self.Set/Reset Tile` false)
    (set `self.Update` false)
    (`SceneComponent.SetVisibility` (`self.CubeHolder`) (`self.Show/HideOverlay`) true)
    (`SceneComponent.SetVisibility` (`self.RadarBandLetter`) (`self.Show/HideOverlay`) true)))

(event `Set/Reset Tile`
  (params (UseGlobal :type Boolean))
  (if UseGlobal
    (bind _asglobal_data_instance (cast `/Game/Blueprints/Global_Data_Instance` (`GameplayStatics.GetGameInstance`)))
    (set `self.SelfState` (`/Game/Blueprints/Global_Data_Instance.Global_TileState` _asglobal_data_instance)))
  (switch `/Game/Blueprints/Enums/Tile_State` (`self.SelfState`) :!label _label
    (:`NewEnumerator3`
      (`SceneComponent.SetVisibility` (`self.RadarBandLetter`) false true)
      (`SceneComponent.SetVisibility` (`self.CubeHolder`) false true)
      (`SceneComponent.SetVisibility` (`self.8x8_radar_mesh_Instanced`) false true)
      (`SceneComponent.SetVisibility` (`self.8x8_radar_lod_Instanced`) false true))
    (:`NewEnumerator0`
      (`self.DetailedSetup`)
      (if (`self.Show/HideOverlay`) :!label _label_2
        (`self.BandSetup` :!label _label_3)))
    (:`NewEnumerator1`
      (`self.PublicSetup`)
      (goto _label_2))
    (:`NewEnumerator2`
      (`SceneComponent.SetVisibility` (`self.8x8_radar_mesh_Instanced`) false true)
      (`SceneComponent.SetVisibility` (`self.8x8_radar_lod_Instanced`) false true)
      (goto _label_3))))

(event `SetupFromVehicle`
  (params (SelfState :type "/Game/Blueprints/Enums/Tile_State Enum" :default "NewEnumerator3") (`Show/HideOverlay` :type Boolean))
  (set `self.SelfState` SelfState)
  (set `self.Show/HideOverlay` `Show/HideOverlay`)
  (goto _label))

(event `ShowBands`
  (`SceneComponent.SetVisibility` (`self.8x8_radar_mesh_Instanced`) false true)
  (`SceneComponent.SetVisibility` (`self.8x8_radar_lod_Instanced`) false true)
  (`SceneComponent.SetVisibility` (`self.CubeHolder`) true true)
  (`SceneComponent.SetVisibility` (`self.RadarBandLetter`) true true))

(event `ChangeLetterAttachPoint`
  (`SceneComponent.K2_AttachToComponent` (`self.RadarBandLetter`) (`self.DefaultSceneRoot`) "None" "KeepWorld" "KeepRelative" "KeepRelative" true))

(fn `BandSetup`
  (locals (SmallestScale :type "Float (double-precision)"))
  (bind _returnvalue (`KismetMathLibrary.Conv_IntToDouble` (`KismetMathLibrary.Min` (`self.RowAmount`) (`self.ColumnAmount`))))
  (`SceneComponent.SetVisibility` (`self.CubeHolder`) true true)
  (`SceneComponent.SetVisibility` (`self.RadarBandLetter`) true true)
  (`PrimitiveComponent.SetMaterial` (`self.RadarBandLetter`) 0 (select `/Game/Blueprints/Enums/BandLetters` (`self.BandLetter`) :`NewEnumerator0` "/Game/_CEARepositoryFiles/3DAssets/Vehicles/RadarTiles/RadarBands/LetterIcons/XBand_Inst.XBand_Inst" :`NewEnumerator2` "/Game/_CEARepositoryFiles/3DAssets/Vehicles/RadarTiles/RadarBands/LetterIcons/CBand_Inst.CBand_Inst" :`NewEnumerator1` "/Game/_CEARepositoryFiles/3DAssets/Vehicles/RadarTiles/RadarBands/LetterIcons/SBand_Inst.SBand_Inst" :`NewEnumerator3` "/Game/_CEARepositoryFiles/3DAssets/Vehicles/RadarTiles/RadarBands/LetterIcons/LBand_Inst.LBand_Inst" :!type "MaterialInterface Object Reference"))
  (`SceneComponent.SetRelativeScale3D` (`self.RadarBandLetter`) (`KismetMathLibrary.MakeVector` 1.0 _returnvalue _returnvalue))
  (`self.CalculateBoxSize` (`self.CubeHolder`))
  (`PrimitiveComponent.SetMaterial` (`self.Cube`) 0 (select `/Game/Blueprints/Enums/BandLetters` (`self.BandLetter`) :`NewEnumerator0` "/Game/_CEARepositoryFiles/3DAssets/Vehicles/RadarTiles/RadarBeams/XBand_Inst.XBand_Inst" :`NewEnumerator2` "/Game/_CEARepositoryFiles/3DAssets/Vehicles/RadarTiles/RadarBeams/CBand_Inst.CBand_Inst" :`NewEnumerator1` "/Game/_CEARepositoryFiles/3DAssets/Vehicles/RadarTiles/RadarBeams/SBand_Inst.SBand_Inst" :`NewEnumerator3` "/Game/_CEARepositoryFiles/3DAssets/Vehicles/RadarTiles/RadarBeams/LBand_Inst.LBand_Inst" :!type "MaterialInterface Object Reference")))

(fn `CalculateBoxSize`
  (params (Object :type "SceneComponent Object Reference"))
  (bind _columnamount (`self.ColumnAmount`))
  (bind _rowamount (`self.RowAmount`))
  (`SceneComponent.SetRelativeScale3D` Object (`KismetMathLibrary.MakeVector` 1.0 (- (`KismetMathLibrary.Conv_IntToDouble` _columnamount) (/ (`KismetMathLibrary.Conv_IntToDouble` _columnamount) 10.0)) (- (`KismetMathLibrary.Conv_IntToDouble` _rowamount) (/ (`KismetMathLibrary.Conv_IntToDouble` _rowamount) 10.0)))))

(fn `DetailedSetup`
  (`SceneComponent.SetVisibility` (`self.RadarBandLetter`) false true)
  (`SceneComponent.SetVisibility` (`self.CubeHolder`) false true)
  (`SceneComponent.SetVisibility` (`self.8x8_radar_lod_Instanced`) false true)
  (`SceneComponent.SetVisibility` (`self.8x8_radar_mesh_Instanced`) true true)
  (`self.SetupTileArray` (`self.8x8_radar_mesh_Instanced`)))

(fn `PublicSetup`
  (`SceneComponent.SetVisibility` (`self.RadarBandLetter`) false true)
  (`SceneComponent.SetVisibility` (`self.CubeHolder`) false true)
  (`SceneComponent.SetVisibility` (`self.8x8_radar_mesh_Instanced`) false true)
  (`SceneComponent.SetVisibility` (`self.8x8_radar_lod_Instanced`) true true)
  (`self.SetupTileArray` (`self.8x8_radar_lod_Instanced`)))

(fn `SetupTileArray`
  (params (Target :type "InstancedStaticMeshComponent Object Reference"))
  (bind _offsetdistance (`self.OffsetDistance`))
  (bind _offsetdistance_2 (`self.OffsetDistance`))
  (bind _returnvalue (/ _offsetdistance_2 2.0))
  (for _index (range (`self.RowAmount`))
    (for _index_2 (range (`self.ColumnAmount`))
      (`InstancedStaticMeshComponent.AddInstance` (`local.Target`) (`KismetMathLibrary.MakeTransform` (`KismetMathLibrary.MakeVector` 0.0 (- (* (`KismetMathLibrary.Conv_IntToDouble` _index_2) _offsetdistance) (- (* (/ (`KismetMathLibrary.Conv_IntToDouble` (`self.ColumnAmount`)) 2.0) _offsetdistance_2) _returnvalue)) (- (* _offsetdistance (`KismetMathLibrary.Conv_IntToDouble` _index)) (- (* (/ (`KismetMathLibrary.Conv_IntToDouble` (`self.RowAmount`)) 2.0) _offsetdistance_2) _returnvalue))))))))

(fn `UserConstructionScript`
  (`self.Set/Reset Tile` false))