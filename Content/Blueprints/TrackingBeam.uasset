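; Beam actor that visually links its location to a Target actor plus offset, following it as either moves.
; A looping timer re-aims two straight spline meshes, with FalloffDistance shortening the beam and proportionally shrinking its end scale.
; SplineMesh uses the behind material and is toggled by BeamInFront, while SplineOnTop is slightly narrower at the end.
; Dynamic materials receive colour on each spline update and opacity every Tick.
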(event `self.ReceiveBeginPlay`
  (`KismetSystemLibrary.K2_SetTimer` self "update spline" (`self.refresh time`) true)
  (`self.update spline`))

(event `self.ReceiveTick`
  (params (DeltaSeconds :type "Float (single-precision)"))
  (`MaterialInstanceDynamic.SetScalarParameterValue` (`self.dynamat`) "Opacity Overide" (`self.Opacity`))
  (`MaterialInstanceDynamic.SetScalarParameterValue` (`self.dynamat_1`) "Opacity Overide" (`self.Opacity`)))

(fn `update spline`
  (bind _returnvalue (`self.K2_GetActorLocation`))
  (bind _splinemesh (`self.SplineMesh`))
  (bind _returnvalue_2 (+ (`self.K2_GetActorLocation` (`self.target`)) (`self.EndPointOffset`)))
  (bind _returnvalue_3 (`KismetMathLibrary.GetDirectionUnitVector` _returnvalue _returnvalue_2))
  (bind _returnvalue_4 (- _returnvalue_2 _returnvalue))
  (bind _returnvalue_5 (- _returnvalue_4 (* _returnvalue_4 (`self.FalloffDistance`))))
  (bind _returnvalue_6 (`KismetMathLibrary.MapRangeClamped` (`KismetMathLibrary.VSize` _returnvalue_5) 0.0 (`KismetMathLibrary.VSize` _returnvalue_4) 0.0 (`self.Scale`)))
  (bind _returnvalue_7 (* _returnvalue_6 0.9))
  (`SplineMeshComponent.SetStartAndEnd` _splinemesh (0.0 0.0 0.0) _returnvalue_3 _returnvalue_5 _returnvalue_3 true)
  (`SplineMeshComponent.SetStartAndEnd` (`self.Spline_OnTop`) (0.0 0.0 0.0) _returnvalue_3 _returnvalue_5 _returnvalue_3 true)
  (`SplineMeshComponent.SetEndScale` _splinemesh (`KismetMathLibrary.MakeVector2D` _returnvalue_6 _returnvalue_6) true)
  (`SplineMeshComponent.SetEndScale` (`self.Spline_OnTop`) (`KismetMathLibrary.MakeVector2D` _returnvalue_7 _returnvalue_7) true)
  (`MaterialInstanceDynamic.SetVectorParameterValue` (`self.dynamat`) "Emissive Colour" (`self.Colour`))
  (`MaterialInstanceDynamic.SetVectorParameterValue` (`self.dynamat_1`) "Emissive Colour" (`self.Colour`)))

(fn `UserConstructionScript`
  (if (`self.Refresh`)
    (set `self.Refresh` false))
  (bind _returnvalue (`PrimitiveComponent.CreateDynamicMaterialInstance` (`self.SplineMesh`) 0 "/Game/_CEARepositoryFiles/_MasterMaterials/Beam_Behind_Inst.Beam_Behind_Inst" "None"))
  (set `self.dynamat` _returnvalue)
  (bind _returnvalue_2 (`PrimitiveComponent.CreateDynamicMaterialInstance` (`self.Spline_OnTop`) 0 "/Game/_CEARepositoryFiles/_MasterMaterials/Beam_MatInst.Beam_MatInst" "None"))
  (set `self.dynamat_1` _returnvalue_2)
  (`self.update spline`)
  (`MaterialInstanceDynamic.SetScalarParameterValue` (`self.dynamat`) "Opacity Overide" (`self.Opacity`))
  (`MaterialInstanceDynamic.SetScalarParameterValue` (`self.dynamat_1`) "Opacity Overide" (`self.Opacity`))
  (`SceneComponent.SetVisibility` (`self.SplineMesh`) (`self.BeamInFront`) false))