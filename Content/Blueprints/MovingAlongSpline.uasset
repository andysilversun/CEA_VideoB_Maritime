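; Spline-following actor that animates an MK-45 shell mesh along an arc, started by its MK-45ShellArc event.
; The ShellArc timeline, with play rate multiplied by Speed, outputs a normalized Distance that is scaled by spline length.
; Each update sets the mesh's world location and relative rotation from the spline at that distance.
; When the timeline finishes, the actor is hidden rather than destroyed.
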(event `MK-45 Shell Arc`
  (bind _spline (`self.Spline`))
  (bind _staticmesh (`self.StaticMesh`))
  (bind _shell_arc (`self.Shell Arc`))
  (`TimelineComponent.SetPlayRate` _shell_arc (* (`TimelineComponent.GetPlayRate` _shell_arc) (`self.Speed`)))
  (bind (_direction _distance) (`Timeline|Shell Arc`)
    (:`Update`
      (bind _returnvalue (* _distance (`SplineComponent.GetSplineLength` _spline)))
      (`SceneComponent.K2_SetWorldLocation` _staticmesh (`SplineComponent.GetLocationAtDistanceAlongSpline` _spline _returnvalue "World") false false)
      (`SceneComponent.K2_SetRelativeRotation` _staticmesh (`SplineComponent.GetRotationAtDistanceAlongSpline` _spline _returnvalue "Local") false false))
    (:`Finished`
      (`self.SetActorHiddenInGame` true))))

(fn `UserConstructionScript`)