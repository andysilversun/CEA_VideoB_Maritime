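; Placeable decal actor that draws two to four concentric coloured range bands marked with letters, plus a radar sphere.
; The construction script sizes bands as percentages of Band4, nudges edited sizes between neighbours, applies dynamic material colours and rings Band_Letters child actors around visible bands.
; At runtime, events toggle decals, letters and sphere.
; Capsule3 overlaps send visibility messages to the overlapping actor.
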(event `self.ReceiveBeginPlay`
  (for _array_element (`self.GetAllChildActors` true)
    (bind _asband_letters (cast `/Game/Blueprints/Band_Letters` _array_element))
    (`KismetArrayLibrary.Array_Add` (`self.LetterList`) _asband_letters)))

(event `Toggle_Letters`
  (params (isVisible :type Boolean))
  (`self.ToggleLetters` isVisible))

(event `Toggle_Radar_Sphere`
  (params (isHidden :type Boolean))
  (`SceneComponent.SetHiddenInGame` (`self.Sphere`) isHidden false))

(event `Turn_Decals_Off`
  (`self.ToggleDecals` true))

(event `Turn_Decals_On`
  (`self.ToggleDecals` false))

(event `self.Capsule3.OnComponentBeginOverlap`
  (params (OverlappedComponent :type "PrimitiveComponent Object Reference") (OtherActor :type "Actor Object Reference") (OtherComp :type "PrimitiveComponent Object Reference") (OtherBodyIndex :type Integer) (bFromSweep :type Boolean) (SweepResult :type "HitResult Structure (by ref)"))
  (message `/Game/Blueprints/Radar_Interactions.Visibility_set` OtherActor true self))

(event `self.Capsule3.OnComponentEndOverlap`
  (params (OverlappedComponent :type "PrimitiveComponent Object Reference") (OtherActor :type "Actor Object Reference") (OtherComp :type "PrimitiveComponent Object Reference") (OtherBodyIndex :type Integer))
  (message `/Game/Blueprints/Radar_Interactions.Visibility_set` OtherActor false self))

(fn `SetBandLetters`
  (switch `/Game/Blueprints/Enums/BandSize` (`self.Number_of_bands`)
    (:`NewEnumerator0`
      _)
    (:`NewEnumerator1`
      (bind _output_get (set `self.Band3_size%` 100.0))
      (set `self.Band3_oldsize` _output_get)
      (`self.SetupLetters` (`self.Band 3`) (`self.Band3_size%`) (`self.Band3_oldsize`) "NewEnumerator1" false (`self.Band3_colour`) :!label _label))
    (:`NewEnumerator2`
      (`self.SetupLetters` (`self.Band 4`) (`self.Band4_size`) (`self.Band4_oldsize`) "NewEnumerator3" true (`self.Band4_colour`))
      (goto _label)))
  (`self.SetupLetters` (`self.Band 2`) (`self.Band2_size%`) (`self.Band2_oldsize`) "NewEnumerator2" false (`self.Band2_colour`))
  (`self.SetupLetters` (`self.Band 1`) (`self.Band1_size%`) (`self.Band1_oldsize`) "NewEnumerator0" false (`self.Band1_colour`))
  (set `self.Last_number_count` (`self.Number_of_Letters`)))

(fn `SetSizes`
  (bind _returnvalue (* (`self.Band4_size`) 0.363636))
  (set `self.Height` (/ (`self.Band4_size`) 2.0))
  (bind _scale (`self.SetupSize` (`self.Band 1`) (`self.Band1_size%`) -1.0 (`self.Band2_size%`) (`self.Band1_oldsize`)))
  (set `self.Band1_size%` _scale)
  (bind _scale_2 (`self.SetupSize` (`self.Band 2`) (`self.Band2_size%`) (`self.Band1_size%`) (`self.Band3_size%`) (`self.Band2_oldsize`)))
  (set `self.Band2_size%` _scale_2)
  (bind _scale_3 (`self.SetupSize` (`self.Band 3`) (`self.Band3_size%`) (`self.Band2_size%`) (`self.Band4_size`) (`self.Band3_oldsize`)))
  (set `self.Band3_size%` _scale_3)
  (`SceneComponent.SetRelativeScale3D` (`self.Band 4`) (`KismetMathLibrary.MakeVector` (`self.Height`) _returnvalue _returnvalue)))

(fn `SetupBands`
  (bind _number_of_bands (`self.Number_of_bands`))
  (if (`|EnumInequality` (`self.Number_of_bands`) (`self.Previous_BandType`))
    (switch `/Game/Blueprints/Enums/BandSize` _number_of_bands
      (:`NewEnumerator0`
        (set `self.Band2_size%` 100.0)
        (`SceneComponent.SetVisibility` (`self.Band 3`) false true)
        (set `self.Band3_size%` 100.0 :!label _label)
        (`SceneComponent.SetVisibility` (`self.Band 4`) false true))
      (:`NewEnumerator1`
        (`SceneComponent.SetVisibility` (`self.Band 3`) true true)
        (set `self.Band2_size%` 50.0)
        (goto _label))
      (:`NewEnumerator2`
        (set `self.Band3_size%` 75.0)
        (`SceneComponent.SetVisibility` (`self.Band 3`) true true)
        (`SceneComponent.SetVisibility` (`self.Band 4`) true true)
        (set `self.Band2_size%` 50.0)))
    (set `self.Band1_size%` 25.0)
    (else
      (switch `/Game/Blueprints/Enums/BandSize` _number_of_bands
        (:`NewEnumerator0`
          (set `self.Band2_size%` 100.0))
        (:`NewEnumerator1`
          _))
      (set `self.Band3_size%` 100.0)
      (`SceneComponent.SetVisibility` (`self.Band 4`) false true))))

(fn `SetupColours`
  (bind _band2_colour (`self.Band2_colour`))
  (bind _band3_colour (`self.Band3_colour`))
  (bind _band4_colour (`self.Band4_colour`))
  (bind _band1_colour (`self.Band1_colour`))
  (`self.SetupMaterial` (`self.Band 1`) (`self.Band1RingDecal`) _band1_colour)
  (`self.SetupMaterial` (`self.Decal1`) (`self.Band1RingDecal`) _band1_colour)
  (`self.SetupMaterial` (`self.Band 2`) (`self.Band2CentreDecal`) _band2_colour)
  (`self.SetupMaterial` (`self.Decal2`) (`self.Band2RingDecal`) _band2_colour)
  (`self.SetupMaterial` (`self.Band 3`) (`self.Band3CentreDecal`) _band3_colour)
  (`self.SetupMaterial` (`self.Decal3`) (`self.Band3RingDecal`) _band3_colour)
  (`self.SetupMaterial` (`self.Band 4`) (`self.Band4CentreDecal`) _band4_colour)
  (`self.SetupMaterial` (`self.Decal4`) (`self.Band4RingDecal`) _band4_colour))

(fn `SetupLetters`
  (params (Decal :type "DecalComponent Object Reference") (distance :type "Float (double-precision)") (old_dist :type "Float (double-precision)") (Letter :type "/Game/Blueprints/Enums/BandLetters Enum" :default "NewEnumerator0") (isLast :type Boolean) (colour :type "LinearColor Structure"))
  (locals (rotateAmount :type "Float (double-precision)"))
  (bind (_colour_r _colour_g _colour_b) (break `LinearColor` (`local.colour`)))
  (bind (_colour_r_2 _colour_g_2 _colour_b_2) (break `LinearColor` (`local.colour`)))
  (bind _returnvalue (* (`KismetMathLibrary.GetUpVector` (struct)) (* (`self.Letter_Height`) 100.0)))
  (bind (_returnvalue_x _returnvalue_y _returnvalue_z) (`KismetMathLibrary.BreakVector` (+ (`KismetMathLibrary.MakeVector` _colour_r _colour_g _colour_b) (`KismetMathLibrary.MakeVector` _colour_r_2 _colour_g_2 _colour_b_2))))
  (if (== distance old_dist)
    (set `local.rotateAmount` (/ 180.0 (`KismetMathLibrary.Conv_IntToDouble` (`self.Number_of_Letters`))))
    (for _index (range (`self.Number_of_Letters`))
      (bind _returnvalue_2 (`AddComponent|NODE_AddChildActorComponent-4` :`RelativeTransform` (`KismetMathLibrary.MakeTransform` (0.0 0.0 0.0) (`KismetMathLibrary.MakeRotator` 0.0 0.0 (* _index (`local.rotateAmount`))))))
      (bind _asband_letters (cast `/Game/Blueprints/Band_Letters` (`ChildActorComponent.ChildActor` _returnvalue_2)))
      (`/Game/Blueprints/Band_Letters.UpdateLetter` _asband_letters (`local.Letter`) (`ActorComponent.GetOwner` (`local.Decal`)) (`KismetMathLibrary.MakeColor` _returnvalue_x _returnvalue_y _returnvalue_z) (`self.Letter_Size`))
      (if (`local.isLast`)
        (bind _returnvalue_3 (`SceneComponent.GetForwardVector` _returnvalue_2))
        (`SceneComponent.K2_AddLocalOffset` _returnvalue_2 (+ (* _returnvalue_3 (* (`local.distance`) 75.0)) _returnvalue) false true)
        (else
          (`SceneComponent.K2_AddLocalOffset` _returnvalue_2 (+ _returnvalue (* _returnvalue_3 (* (* (/ (`self.Band4_size`) 100.0) (`local.distance`)) 75.0))) false true))))))

(fn `SetupMaterial`
  (params (decal :type "DecalComponent Object Reference") (material :type "MaterialInstance Object Reference") (colour :type "LinearColor Structure"))
  (bind _returnvalue (`DecalComponent.CreateDynamicMaterialInstance` decal))
  (`|VariableSetRef` material material)
  (`MaterialInstanceDynamic.SetVectorParameterValue` _returnvalue "Colour" colour))

(fn `SetupSize`
  (params (Band :type "DecalComponent Object Reference") (size :type "Float (double-precision)") (PreviousBand :type "Float (double-precision)" :default -1.0) (NextBand :type "Float (double-precision)" :default -1.0) (prevSize :type "Float (double-precision)"))
  (returns (scale :type "Float (double-precision)"))
  (locals (newSIze :type "Float (double-precision)"))
  (bind _returnvalue (* (* (/ (`self.Band4_size`) 100.0) (`local.newSIze`)) 0.363636))
  (set `local.newSIze` size)
  (if (and (<= (`local.size`) PreviousBand) (!= prevSize (`local.size`)))
    (set `local.newSIze` (+ (`local.PreviousBand`) 1.0))
    (elif (== (`local.NextBand`) (`self.Band4_size`))
      (if (== (`local.size`) 100.0)
        (set `local.newSIze` 99.0))
      (elif (and (>= (`local.size`) (`local.NextBand`)) (!= (`local.prevSize`) (`local.size`)))
        (set `local.newSIze` (- (`local.NextBand`) 1.0)))))
  (`SceneComponent.SetRelativeScale3D` (`local.Band`) (`KismetMathLibrary.MakeVector` (`self.Height`) _returnvalue _returnvalue))
  (return (`local.newSIze`)))

(fn `ToggleDecals`
  (params (isHidden :type Boolean))
  (`SceneComponent.SetHiddenInGame` (`self.Band 1`) isHidden false)
  (`SceneComponent.SetHiddenInGame` (`self.Band 2`) isHidden false)
  (`SceneComponent.SetHiddenInGame` (`self.Band 3`) isHidden false)
  (`SceneComponent.SetHiddenInGame` (`self.Band 4`) isHidden false)
  (`SceneComponent.SetHiddenInGame` (`self.Decal2`) isHidden false)
  (`SceneComponent.SetHiddenInGame` (`self.Decal3`) isHidden false)
  (`SceneComponent.SetHiddenInGame` (`self.Decal4`) isHidden false)
  (`SceneComponent.SetHiddenInGame` (`self.Decal1`) isHidden false))

(fn `ToggleLetters`
  (params (NewHidden :type Boolean))
  (for _array_element (`self.LetterList`)
    (`SceneComponent.SetHiddenInGame` (`/Game/Blueprints/Band_Letters.DefaultSceneRoot` _array_element) NewHidden false)))

(fn `UserConstructionScript`
  (bind _returnvalue (* (`self.Band4_size`) 1.57))
  (`self.SetupBands`)
  (set `self.Previous_BandType` (`self.Number_of_bands`))
  (`self.SetupColours`)
  (`self.SetSizes`)
  (`self.SetBandLetters`)
  (`self.SetupBands`)
  (bind _output_get (set `self.Band1_oldsize` (`self.Band1_size%`)))
  (bind _output_get_2 (set `self.Band2_oldsize` (`self.Band2_size%`)))
  (bind _output_get_3 (set `self.Band3_oldsize` (`self.Band3_size%`)))
  (bind _output_get_4 (set `self.Band4_oldsize` (`self.Band4_size`)))
  (set `self.Redraw Letters` false)
  (`SceneComponent.SetRelativeScale3D` (`self.Sphere`) (`KismetMathLibrary.MakeVector` _returnvalue _returnvalue _returnvalue)))