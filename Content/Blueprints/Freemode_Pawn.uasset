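; Free-mode pawn that controls level sequence playback, camera view and visibility of scene markers such as decals, letters and icons.
; Keys and callable events share logic to step a clamped play-mode index from triple forward through pause to triple reverse, updating an animated state widget.
; Right mouse toggles a control-widget overlay with matching cursor and input mode, while M blends between pawn and overview camera.
; BeginPlay creates the state widget and disables input.
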(event `Hide_Decals`
  (params (isHidden :type Boolean))
  (bind _outactors (`GameplayStatics.GetAllActorsOfClass` "/Game/Blueprints/Decal_actor.Decal_actor_C"))
  (for _array_element _outactors
    (`/Game/Blueprints/Decal_actor.ToggleDecals` _array_element isHidden)
    (`/Game/Blueprints/Decal_actor.Toggle_Radar_Sphere` _array_element isHidden))
  (bind _outactors_2 (`GameplayStatics.GetAllActorsOfClass` "/Game/Blueprints/Band_Letters.Band_Letters_C"))
  (for _array_element_2 _outactors_2
    (`/Game/Blueprints/Band_Letters.hide_letter` _array_element_2 isHidden)))

(event `Hide_icons`
  (params (NewHidden :type Boolean))
  (bind _outactors (`GameplayStatics.GetAllActorsOfClass` "/Game/Blueprints/icon.icon_C"))
  (for _array_element _outactors
    (`/Game/Blueprints/icon.hide_Icon` _array_element NewHidden)))

(event `self.ReceiveBeginPlay`
  (bind _returnvalue (`|CreateWidget` "/Game/Blueprints/Play_state.Play_state_C"))
  (`UserWidget.AddToViewport` _returnvalue 0)
  (set `self.Play_state_widget` _returnvalue)
  (`self.DisableInput` (`GameplayStatics.GetPlayerController` 0)))

(event `Add controlls`
  (bind (_returnvalue_x _returnvalue_y) (`KismetMathLibrary.BreakVector2D` (`WidgetLayoutLibrary.GetViewportSize`)))
  (bind _returnvalue (`GameplayStatics.GetPlayerController` 0))
  (bind _returnvalue_2 (`|CreateWidget` "/Game/Blueprints/Sequence_controll_module.Sequence_controll_module_C" :!label _label))
  (bind _output_get (set `self.control widget` _returnvalue_2))
  (set `self.overlay_visable` true)
  (if (`self.overlay_visable`) :!label _label_2
    (`UserWidget.AddToViewport` _output_get 0)
    (set `PlayerController.bShowMouseCursor` true _returnvalue)
    (`WidgetBlueprintLibrary.SetInputMode_GameAndUIEx` _returnvalue (`self.control widget`) "DoNotLock" false)
    (`PlayerController.SetMouseLocation` _returnvalue (/ (`KismetMathLibrary.FTrunc` _returnvalue_x) 2) (/ (`KismetMathLibrary.FTrunc` _returnvalue_y) 2))
    (else
      (`Widget.RemoveFromParent` _output_get :!label _label_3)
      (set `PlayerController.bShowMouseCursor` false _returnvalue)
      (`WidgetBlueprintLibrary.SetInputMode_GameOnly` _returnvalue)
      (`WidgetBlueprintLibrary.SetFocusToGameViewport`))))

(event `HUD Toggle`
  (if (`self.overlay_visable`) :!label _label_4
    (set `self.overlay_visable` false)
    (else
      (set `self.overlay_visable` true)))
  (`/Engine/EditorBlueprintResources/StandardMacros.IsValid` (stale `Add controlls` _output_get)
    (:`Is Valid`
      (goto _label_2))
    (:`Is Not Valid`
      (goto _label))))

(event `Key|RightMouseButton`
  (params (Key :type "Key Structure"))
  (:`Pressed`
    (goto _label_4)))

(event `remove controlls`
  (set `self.overlay_visable` false)
  (goto _label_3))

(event `play/pause`
  (bind _play_state_widget (`self.Play_state_widget`))
  (bind _returnvalue (select `int` (`self.Play_mode_index`) :`0` "NewEnumerator2" :`1` "NewEnumerator1" :`2` "NewEnumerator0" :`3` "NewEnumerator3" :`4` "NewEnumerator4" :`5` "NewEnumerator5" :`6` "NewEnumerator6" :!type "/Game/Blueprints/Enums/Sequencer_Play_modes Enum"))
  (bind _sequenceplayer (`LevelSequenceActor.SequencePlayer` (`self.Sequence_controller`)))
  (if (!= (`self.Play_mode_index`) 3) :!label _label_5
    (set `self.Play_mode_index` 3)
    (else
      (set `self.Play_mode_index` 2)))
  (switch `/Game/Blueprints/Enums/Sequencer_Play_modes` _returnvalue :!label _label_6
    (:`NewEnumerator2`
      (`MovieSceneSequencePlayer.SetPlayRate` _sequenceplayer 3.0)
      (`/Engine/EditorBlueprintResources/StandardMacros.IsValid` _sequenceplayer :!label _label_7
        (:`Is Valid`
          (`MovieSceneSequencePlayer.Play` _sequenceplayer))))
    (:`NewEnumerator1`
      (`MovieSceneSequencePlayer.SetPlayRate` _sequenceplayer 2.0)
      (goto _label_7))
    (:`NewEnumerator0`
      (`MovieSceneSequencePlayer.SetPlayRate` _sequenceplayer 1.0)
      (goto _label_7))
    (:`NewEnumerator3`
      (`/Engine/EditorBlueprintResources/StandardMacros.IsValid` _sequenceplayer
        (:`Is Valid`
          (`MovieSceneSequencePlayer.Pause` _sequenceplayer))))
    (:`NewEnumerator4`
      (`MovieSceneSequencePlayer.SetPlayRate` _sequenceplayer -1.0)
      (goto _label_7))
    (:`NewEnumerator5`
      (`MovieSceneSequencePlayer.SetPlayRate` _sequenceplayer -2.0)
      (goto _label_7))
    (:`NewEnumerator6`
      (`MovieSceneSequencePlayer.SetPlayRate` _sequenceplayer -3.0)
      (goto _label_7)))
  (set `/Game/Blueprints/Play_state.play_state` (`KismetTextLibrary.Conv_StringToText` (`|GetEnumeratorNameAsString` _returnvalue)) _play_state_widget)
  (`UserWidget.PlayAnimation` _play_state_widget (`/Game/Blueprints/Play_state.State_update` _play_state_widget) 0.0 1 "Forward" 1.0))

(event `Key|Enter`
  (params (Key :type "Key Structure"))
  (:`Pressed`
    (goto _label_5)))

(event `forward`
  (set `self.Play_mode_index` (`KismetMathLibrary.Clamp` (+ (`self.Play_mode_index`) -1) 0 6) :!label _label_8)
  (goto _label_6))

(event `Key|RightBracket`
  (params (Key :type "Key Structure"))
  (:`Pressed`
    (goto _label_8)))

(event `Key|LeftBracket`
  (params (Key :type "Key Structure"))
  (:`Pressed`
    (set `self.Play_mode_index` (`KismetMathLibrary.Clamp` (+ (`self.Play_mode_index`) 1) 0 6) :!label _label_9)
    (goto _label_6)))

(event `backward`
  (goto _label_9))

(event `Key|M`
  (params (Key :type "Key Structure"))
  (bind _returnvalue (`GameplayStatics.GetPlayerController` 0))
  (:`Pressed`
    (`/Engine/EditorBlueprintResources/StandardMacros.FlipFlop` :!label _label_10
      (:`A`
        (`PlayerController.SetViewTargetWithBlend` _returnvalue (`self.overview_cam`) 1.0 "VTBlend_Linear" 0.0 false))
      (:`B`
        (`PlayerController.SetViewTargetWithBlend` _returnvalue (`GameplayStatics.GetPlayerPawn` 0) 1.0 "VTBlend_Linear" 0.0 false)))))

(event `Overview`
  (goto _label_10))

(fn `UserConstructionScript`)