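; Hawkei vehicle turntable child Blueprint that extends its parent's radar display with CEATAC-specific materials and dust effects.
; Material change and texture swap events set the CEATAC rig to default or camo; transparent variants sit in unexecuted nodes.
; Tick drives two particle systems' speed and colour from movement speed and dust colour.
; Construction assigns the rig and vehicle mesh as radar references before running parent setup.
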(event `self.Isolate_radar`
  (`parent.Isolate_radar`))

(event `self.ForceMatChange`
  (params (Type :type "/Game/Blueprints/Enums/VehicleMaterialType Enum" :default "NewEnumerator0"))
  (bind (_base _camo) (break `/Game/Blueprints/VehicleMaterials` (`self.CEATAC_Materials`)))
  (`parent.ForceMatChange` Type)
  (if (`self.isTransparent`) :!label _label
    _
    (else
      _))
  (`PrimitiveComponent.SetMaterial` (`self.CEATAC_Rigged`) 0 (select `/Game/Blueprints/Enums/VehicleMaterialType` (`self.MaterialType`) :`NewEnumerator0` _base :`NewEnumerator1` _camo)))

(event `self.Swap_textures`
  (`parent.Swap_textures`)
  (goto _label))

(event `self.ReceiveTick`
  (params (DeltaSeconds :type "Float (single-precision)"))
  (`ParticleSystemComponent.SetFloatParameter` (`self.ParticleSystem1`) "Speed" (`KismetMathLibrary.MapRangeUnclamped` (`self.Movement_Speed Km/h`) 0.0 25.0 0.0 1.0))
  (`ParticleSystemComponent.SetFloatParameter` (`self.ParticleSystem`) "Speed" (`KismetMathLibrary.MapRangeUnclamped` (`self.Movement_Speed Km/h`) 0.0 25.0 0.0 1.0))
  (`ParticleSystemComponent.SetColorParameter` (`self.ParticleSystem`) "Colour" (`self.Dust_colour`))
  (`ParticleSystemComponent.SetColorParameter` (`self.ParticleSystem1`) "Colour" (`self.Dust_colour`))
  (`parent.ReceiveTick` DeltaSeconds))

(fn `UserConstructionScript`
  (set `self.RadarRef1` (`self.CEATAC_Rigged`))
  (set `self.RadarRef2` (`self.Vehicle_Skel_Mesh1`))
  (`parent.UserConstructionScript`))