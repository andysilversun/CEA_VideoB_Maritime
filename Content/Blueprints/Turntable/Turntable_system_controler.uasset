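; Turntable controller actor that swaps the displayed vehicle and its surrounding environment.
; Spawning kills the current vehicle and creates the one found in the Vehicle array, offsetting the trailer.
; Environments are streamed levels cycled by looping MultiGates per MODE (land: showroom, bush, desert; maritime: showroom, ocean), with force events for direct selection.
; Switches update EnviroIndex, showing the static mesh in showrooms and hiding it for bush and ocean.
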(event `spawn_ vehicle`
  (params (ItemToFind :type "/Game/Blueprints/Turntable/Base_Vehicle Class Reference (by ref)"))
  (bind _vehicle (`self.vehicle`))
  (bind _current_vehicle (`self.current vehicle`))
  (bind _returnvalue (`KismetArrayLibrary.Array_Find` _vehicle ItemToFind))
  (bind _output (`|GetArrayItem` _vehicle _returnvalue))
  (`/Engine/EditorBlueprintResources/StandardMacros.IsValid` _current_vehicle
    (:`Is Valid`
      (`/Game/Blueprints/Turntable/Base_Vehicle.Kill` _current_vehicle))
    (:`Is Not Valid`
      _))
  (if (== _returnvalue -1)
    (`KismetSystemLibrary.PrintString` "ERROR: Vehicle not found")
    (else
      (bind _returnvalue_2 (`|SpawnActorFromClass` _output (`KismetMathLibrary.MakeTransform` (+ (0.0 0.0 2.5) (select `bool` (== _output "/Game/Blueprints/Turntable/Trailer_Turntable.Trailer_Turntable_C") :`true` (224.0 0.0 0.0) :!type "Vector Structure"))) "AlwaysSpawn" "OverrideRootScale" null null))
      (set `self.current vehicle` _returnvalue_2))))

(event `self.ReceiveBeginPlay`
  (bind _mode (`self.MODE`))
  (`SceneComponent.SetHiddenInGame` (`self.StaticMeshComponent`) false false :!label _label)
  (`GameplayStatics.LoadStreamLevel` (select `/Game/Blueprints/Enums/TurntableType` _mode :`NewEnumerator0` "Turntable_Showroom" :`NewEnumerator1` "Turntable_MaritimeShowroom" :!type "Name") true)
  (`GameplayStatics.UnloadStreamLevel` (select `/Game/Blueprints/Enums/TurntableType` _mode :`NewEnumerator0` "Turntable_Desert" :`NewEnumerator1` "Turntable_Ocean" :!type "Name")))

(event `force showroom environ`
  (set `self.Enviro_index` 1 :!label _label_2)
  (goto _label))

(event `force forest environment`
  (set `self.Enviro_index` 2 :!label _label_3)
  (`SceneComponent.SetHiddenInGame` (`self.StaticMeshComponent`) true false)
  (`GameplayStatics.LoadStreamLevel` "Turntable_Bush" true)
  (`GameplayStatics.UnloadStreamLevel` "Turntable_Showroom"))

(event `toggle environment`
  (switch `/Game/Blueprints/Enums/TurntableType` (`self.MODE`)
    (:`NewEnumerator0`
      (`|MultiGate` false true 1
        (:`Out 0`
          (goto _label_2))
        (:`Out 1`
          (goto _label_3))
        (:`Out 2`
          (set `self.Enviro_index` 3 :!label _label_4)
          (`GameplayStatics.LoadStreamLevel` "Turntable_Desert" true)
          (`GameplayStatics.UnloadStreamLevel` "Turntable_Bush"))))
    (:`NewEnumerator1`
      (`|MultiGate` false true 1
        (:`Out 0`
          (goto _label_2))
        (:`Out 1`
          (set `self.Enviro_index` 2 :!label _label_5)
          (`SceneComponent.SetHiddenInGame` (`self.StaticMeshComponent`) true false)
          (`GameplayStatics.LoadStreamLevel` "Turntable_Ocean" true)
          (`GameplayStatics.UnloadStreamLevel` "Turntable_MaritimeShowroom"))))))

(event `force_desert_environ`
  (goto _label_4))

(event `force ocean environment`
  (goto _label_5))

(event `set time`
  (params (time :type "Float (double-precision)"))
  (set `self.time` time))

(fn `UserConstructionScript`)