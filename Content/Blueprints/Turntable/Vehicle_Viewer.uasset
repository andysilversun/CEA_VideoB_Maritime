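; Radar vehicle display actor that either spins on a turntable or drives along a spline, depending on IsTurnTableMode.
; Turntable features include material cycling, animation playback, a zoom-driven component spread, and radar isolation that makes the vehicle invisible and relocates the pawn.
; Spline movement derives speed from path timing.
; Land and water units snap to traced ground, with land units tilting to averaged normals, while aircraft take spline positions directly.
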(event `self.ReceiveBeginPlay`
  (bind _anim_ui (`self.anim_ui`))
  (bind _asturntable_pawn (cast `/Game/Blueprints/Turntable/Turntable_Pawn` (`GameplayStatics.GetPlayerPawn` 0))
    (:`then`
      (bind _output_get (set `self.pawn` _asturntable_pawn))
      (`self.change_zoom` (`KismetMathLibrary.MapRangeClamped` (`/Game/Blueprints/Turntable/Turntable_Pawn.Spring arm length` _output_get) 200.0 1300.0 0.0 1.0))
      (`/Game/Blueprints/Turntable/Turntable_Pawn.hide idle` _output_get)
      (`/Game/Blueprints/Turntable/Turntable_Pawn.drag screen messege` _output_get)
      (bind _foundwidgets (`WidgetBlueprintLibrary.GetAllWidgetsOfClass` "/Game/Blueprints/Turntable/TurnTable_Anim_UI.TurnTable_Anim_UI_C" false))
      (bind _output (`|GetArrayItem` _foundwidgets))
      (`/Engine/EditorBlueprintResources/StandardMacros.IsValid` _output
        (:`Is Valid`
          (set `self.anim_ui` _output))
        (:`Is Not Valid`
          (bind _returnvalue (`|CreateWidget` "/Game/Blueprints/Turntable/TurnTable_Anim_UI.TurnTable_Anim_UI_C"))
          (set `self.anim_ui` _returnvalue)
          (`UserWidget.AddToViewport` _anim_ui 1)))
      (message `/Game/Blueprints/Turntable/Anim_IF.setup anim` (`SkeletalMeshComponent.GetAnimInstance` (`self.Radar_Skel_Mesh`)) _anim_ui))
    (:`CastFailed`
      (set `self.isTurnTableMode` false)))
  (`SceneComponent.SetVisibility` (`self.Radar_component_group`) false true)
  (`SceneComponent.SetVisibility` (`self.Secondary_Radar_component_group`) false true)
  (`SceneComponent.SetVisibility` (`self.Tertiary_Radar_component_group`) false true)
  (set `self.isTransparent` true)
  (`self.Isolate_radar`)
  (`KismetSystemLibrary.Delay` 0.2)
  (bind _returnvalue_2 (`|SpawnActorFromClass` (`self.Stats`) (`KismetMathLibrary.MakeTransform` (0.0 0.0 0.0)) "Undefined" "OverrideRootScale" null null))
  (set `self.StatsRef` _returnvalue_2)
  (`self.K2_SetActorLocation` (`GameplayStatics.GetPlayerPawn` 0) (`SceneComponent.K2_GetComponentLocation` (`self.Main_Cam`)) false false)
  (set `self.TimeToCompletePath` (+ (* (/ (`self.Vehicle_Target_Distance`) (`self.Vehicle_Speed`)) 3600.0) (`self.TimeToStartPath`)))
  (`KismetSystemLibrary.Delay` 0.1)
  (`self.UnitSetup`))

(event `self.ReceiveTick`
  (params (DeltaSeconds :type "Float (single-precision)"))
  (if (`self.isTurnTableMode`)
    (if (`self.isAutoRotate`)
      (`SceneComponent.K2_AddLocalRotation` (`self.Vehicle_Skel_Mesh1`) (* (struct :`Yaw` 1.0) (* DeltaSeconds (`self.RotateSpeed`))) false false))
    (else
      (`self.Movement`))))

(event `self.Rotate`
  (params (Automated :type Boolean) (Speed :type "Float (single-precision)") (Custom_Angle :type "Float (single-precision)"))
  (set `self.isAutoRotate` Automated)
  (set `self.RotateSpeed` (`KismetMathLibrary.FClamp` (+ (`self.RotateSpeed`) Speed) -360.0 360.0)))

(event `self.Isolate_radar`
  (bind _material_index (`self.Material_Index`))
  (bind _material_index_2 (`self.Material_Index`))
  (bind _output_get (set `self.isTransparent` (not (`self.isTransparent`))))
  (if _output_get
    (`self.ToggleIsolation` true (`self.Material_Invisible`) (`|GetArrayItem` (`self.Radar_Transl_Material_List`) _material_index) (`|GetArrayItem` (`self.Secondary_Radar_Transl_Material_List`) _material_index) (`SceneComponent.K2_GetComponentLocation` (`self.Radar_Cam`)))
    (else
      (`self.ToggleIsolation` false (`|GetArrayItem` (`self.Material_List`) (`self.Material_Index`)) (`|GetArrayItem` (`self.Radar_Material_List`) _material_index_2) (`|GetArrayItem` (`self.Secondary_Radar_Material_List`) _material_index_2) (`SceneComponent.K2_GetComponentLocation` (`self.Main_Cam`))))))

(event `ForceMatChange`
  (params (Index :type Integer))
  (bind _radar_skel_mesh_2 (`self.Radar_Skel_Mesh_2`))
  (bind _material_index (`self.Material_Index`))
  (bind _vehicle (`self.Vehicle`))
  (bind _secondary_mesh (`self.Secondary_Mesh`))
  (bind _material_index_2 (`self.Material_Index`))
  (bind _radar_skel_mesh_2_2 (`self.Radar_Skel_Mesh_2`))
  (bind _radar_skel_mesh (`self.Radar_Skel_Mesh`))
  (bind _vehicle_2 (`self.Vehicle`))
  (bind _secondary_mesh_2 (`self.Secondary_Mesh`))
  (bind _output (`|GetArrayItem` (`self.Secondary_Radar_Material_List`) _material_index_2))
  (bind _output_2 (`|GetArrayItem` (`self.Radar_Transl_Material_List`) _material_index))
  (bind _output_3 (`|GetArrayItem` (`self.Secondary_Radar_Transl_Material_List`) _material_index))
  (set `self.Material_Index` Index)
  (if (> (stale `self.Swap_textures` _result) (- (`KismetArrayLibrary.Array_Length` (`self.Material_List`)) 1)) :!label _label
    (set `self.Material_Index` 0))
  (if (`self.isTransparent`)
    (`/Engine/EditorBlueprintResources/StandardMacros.IsValid` _output_2
      (:`Is Valid`
        (`PrimitiveComponent.SetMaterial` (`self.Radar_Skel_Mesh`) 0 _output_2))
      (:`Is Not Valid`
        _))
    (`/Engine/EditorBlueprintResources/StandardMacros.IsValid` _radar_skel_mesh_2_2
      (:`Is Valid`
        (`PrimitiveComponent.SetMaterial` _radar_skel_mesh_2_2 0 _output_3))
      (:`Is Not Valid`
        _))
    (`/Engine/EditorBlueprintResources/StandardMacros.IsValid` _secondary_mesh_2
      (:`Is Valid`
        (`PrimitiveComponent.SetMaterial` _secondary_mesh_2 0 _output_3))
      (:`Is Not Valid`
        _))
    (`/Engine/EditorBlueprintResources/StandardMacros.IsValid` _vehicle_2
      (:`Is Valid`
        (`PrimitiveComponent.SetMaterial` _vehicle_2 0 (`self.Material_Invisible`))))
    (else
      (`PrimitiveComponent.SetMaterial` (`self.Vehicle_Skel_Mesh1`) 0 (`|GetArrayItem` (`self.Material_List`) _material_index_2))
      (`/Engine/EditorBlueprintResources/StandardMacros.IsValid` _radar_skel_mesh
        (:`Is Valid`
          (`PrimitiveComponent.SetMaterial` _radar_skel_mesh 0 (`|GetArrayItem` (`self.Radar_Material_List`) _material_index_2)))
        (:`Is Not Valid`
          _))
      (`/Engine/EditorBlueprintResources/StandardMacros.IsValid` _radar_skel_mesh_2
        (:`Is Valid`
          (`PrimitiveComponent.SetMaterial` _radar_skel_mesh_2 0 _output))
        (:`Is Not Valid`
          _))
      (`/Engine/EditorBlueprintResources/StandardMacros.IsValid` _secondary_mesh
        (:`Is Valid`
          (`PrimitiveComponent.SetMaterial` _secondary_mesh 0 _output))
        (:`Is Not Valid`
          _))
      (`/Engine/EditorBlueprintResources/StandardMacros.IsValid` _vehicle
        (:`Is Valid`
          (`PrimitiveComponent.SetMaterial` _vehicle 0 (`|GetArrayItem` (`self.Material_List`) _material_index_2)))))))

(event `self.Swap_textures`
  (bind _result (`/Engine/EditorBlueprintResources/StandardMacros.IncrementInt` (`self.Material_Index`))
    (:`  `
      (goto _label))))

(event `Kill`
  (bind _statsref (`self.StatsRef`))
  (`/Engine/EditorBlueprintResources/StandardMacros.IsValid` _statsref
    (:`Is Valid`
      (`self.K2_DestroyActor` _statsref)
      (`KismetSystemLibrary.Delay` 0.1))
    (:`Is Not Valid`
      _))
  (`self.K2_DestroyActor`))

(event `self.Play/Pause Anim`
  (bind _anim_ui (`self.anim_ui`))
  (bind _radar_skel_mesh (`self.Radar_Skel_Mesh`))
  (bind _returnvalue (`SkeletalMeshComponent.GetAnimInstance` _radar_skel_mesh))
  (`/Engine/EditorBlueprintResources/StandardMacros.IsValid` _radar_skel_mesh
    (:`Is Valid`
      (if (`self.Multi_mode`)
        (message `/Game/Blueprints/Turntable/Anim_IF.Set_play_mode` _returnvalue _anim_ui)
        (else
          (`/Engine/EditorBlueprintResources/StandardMacros.FlipFlop`
            (:`A`
              (message `/Game/Blueprints/Turntable/Anim_IF.Set_Play_rate` _returnvalue -1.0 _anim_ui))
            (:`B`
              (message `/Game/Blueprints/Turntable/Anim_IF.Set_Play_rate` _returnvalue 1.0 _anim_ui))))))))

(event `deploy/stow stands`
  (params (forward :type Boolean))
  (bind _vehicle_skel_mesh1 (`self.Vehicle_Skel_Mesh1`))
  (if forward
    (`SkeletalMeshComponent.SetPlayRate` _vehicle_skel_mesh1 1.0)
    (else
      (`SkeletalMeshComponent.SetPlayRate` _vehicle_skel_mesh1 -1.0)))
  (`SkeletalMeshComponent.Play` _vehicle_skel_mesh1 false))

(event `change_zoom`
  (params (Alpha :type "Float (double-precision)"))
  (for (_array_element _array_index) (`|MakeArray` (`self.MEG`) (`self.ENV`) (`self.PWR`) (`self.ARY`) (`self.GEN`))
    (`/Engine/EditorBlueprintResources/StandardMacros.IsValid` _array_element
      (:`Is Valid`
        (`SceneComponent.K2_SetRelativeLocation` _array_element (`KismetMathLibrary.VLerp` (`|GetArrayItem` (`self.start point origins`) _array_index) (`SceneComponent.RelativeLocation` (`|GetArrayItem` (`|MakeArray` (`self.alt_start_point`) (`self.alt_start_point2`) (`self.alt_start_point3`) (`self.alt_start_point4`) (`self.alt_start_point5`)) _array_index)) Alpha) false false)))))

(fn `CalculateNewUp`
  (returns (newNormal :type "Vector Structure"))
  (for _index (range (`KismetArrayLibrary.Array_Length` (`self.GroundRayList`)))
    (bind _returnvalue (+ (`|GetArrayItem` (`self.GroundRayList`) _index) (`SceneComponent.K2_GetComponentLocation` (`self.Vehicle`))))
    (bind _outhit (`KismetSystemLibrary.LineTraceSingleForObjects` _returnvalue (- _returnvalue (0.0 0.0 1000.0)) (`|MakeArray` "ObjectTypeQuery1" :!type "EObjectTypeQuery Enum")))
    (set `self.NewUpDir` (+ (`self.NewUpDir`) (`.ImpactNormal` (`GameplayStatics.BreakHitResult` _outhit)))))
  (return (`KismetMathLibrary.Normal` (`self.NewUpDir`))))

(fn `LandSeaRotation`
  (bind _returnvalue (`SplineComponent.GetLocationAtDistanceAlongSpline` (`/Game/Blueprints/WayPoint.Spline` (`self.SplineBP`)) (+ (`self.DistanceAlongSpline`) 100.0) "World"))
  (bind _outhit (`KismetSystemLibrary.LineTraceSingleForObjects` _returnvalue (- _returnvalue (0.0 0.0 10000.0)) (`|MakeArray` "ObjectTypeQuery1" :!type "EObjectTypeQuery Enum")))
  (switch `/Game/Blueprints/Enums/VehicleType` (`self.VehicleType`)
    (:`NewEnumerator0`
      ;[1 1 1] Land Rotation
      (bind _newnormal (`self.CalculateNewUp`))
      (bind _returnvalue_2 (`KismetMathLibrary.Normal` (- (`.ImpactPoint` (`GameplayStatics.BreakHitResult` _outhit)) (`SceneComponent.K2_GetComponentLocation` (`self.DefaultSceneRoot`)))))
      (`SceneComponent.K2_SetWorldRotation` (`self.DefaultSceneRoot`) (`KismetMathLibrary.MakeRotFromZX` _newnormal _returnvalue_2) false false))
    (:`NewEnumerator1`
      ;[1 1 1] Boat Rotation
      (`SceneComponent.K2_SetWorldRotation` (`self.DefaultSceneRoot`) (`KismetMathLibrary.Conv_VectorToRotator` _returnvalue_2) false false))))

(fn `Movement`
  (set `self.DistanceAlongSpline` (+ (* (`GameplayStatics.GetWorldDeltaSeconds`) (* (`self.PlaySpeed`) (`self.Movement_Speed`))) (`self.DistanceAlongSpline`)))
  (`self.SetPosition`)
  (`self.SetRotation`)
  (set `self.LastLocation` (`SceneComponent.K2_GetComponentLocation` (`self.DefaultSceneRoot`))))

(fn `SetPosition`
  (bind _returnvalue (`SplineComponent.GetLocationAtDistanceAlongSpline` (`/Game/Blueprints/WayPoint.Spline` (`self.SplineBP`)) (`self.DistanceAlongSpline`) "World"))
  (switch `/Game/Blueprints/Enums/VehicleType` (`self.VehicleType`)
    (:`NewEnumerator0`
      (bind _outhit (`KismetSystemLibrary.LineTraceSingleForObjects` _returnvalue (- _returnvalue (0.0 0.0 10000.0)) (`|MakeArray` "ObjectTypeQuery1" :!type "EObjectTypeQuery Enum") :!label _label))
      (`SceneComponent.K2_SetWorldLocation` (`self.DefaultSceneRoot`) (`.Location` (`GameplayStatics.BreakHitResult` _outhit)) false false))
    (:`NewEnumerator1`
      (goto _label))
    (:`NewEnumerator2`
      (`SceneComponent.K2_SetWorldLocation` (`self.DefaultSceneRoot`) _returnvalue false false :!label _label_2))
    (:`NewEnumerator3`
      (goto _label_2))))

(fn `SetRotation`
  (if (< (`self.DistanceAlongSpline`) (`SplineComponent.GetSplineLength` (`/Game/Blueprints/WayPoint.Spline` (`self.SplineBP`))))
    (if (< (`self.DistanceAlongSpline`) 0.0)
      ;[1 1 1] Before moving starts
      (`SceneComponent.K2_SetWorldRotation` (`self.DefaultSceneRoot`) (`KismetMathLibrary.Conv_VectorToRotator` (* (`KismetMathLibrary.Normal` (`SplineComponent.GetLocationAtDistanceAlongSpline` (`/Game/Blueprints/WayPoint.Spline` (`self.SplineBP`)) 10.0 "World")) -1)) false false)
      (else
        (switch `/Game/Blueprints/Enums/VehicleType` (`self.VehicleType`)
          (:`NewEnumerator0`
            _)
          (:`NewEnumerator1`
            _))
        (`self.LandSeaRotation`)))))

(fn `StoreSplinePoints`
  (bind _pointinfo (`self.PointInfo`))
  (bind _spline (`/Game/Blueprints/WayPoint.Spline` (`self.SplineBP`)))
  (for _index (range (`SplineComponent.GetNumberOfSplinePoints` _spline))
    (if (< _index (`KismetArrayLibrary.Array_Length` _pointinfo))
      (if (`|EnumEquality` (`.Action_11_86D8DEFF4DFBE2E260EC2AA4693510AD` (break `/Game/Blueprints/SplineStruct` (`|GetArrayItem` _pointinfo _index))) "NewEnumerator3")
        (`KismetArrayLibrary.Array_Add` _pointinfo (make `/Game/Blueprints/SplineStruct` _index (`SplineComponent.GetDistanceAlongSplineAtSplinePoint` _spline _index) "NewEnumerator3") :!label _label))
      (else
        (goto _label)))))

(fn `ToggleIsolation`
  (params (isHidden :type Boolean) (vehicleMat :type "MaterialInstance Object Reference") (radarMat :type "MaterialInstance Object Reference") (secondRadarMat :type "MaterialInstance Object Reference") (cameraLoc :type "Vector Structure"))
  (bind _returnvalue (`GameplayStatics.GetPlayerPawn` 0))
  (bind _radar_skel_mesh_2 (`self.Radar_Skel_Mesh_2`))
  (bind _secondary_mesh (`self.Secondary_Mesh`))
  (bind _radar_skel_mesh (`self.Radar_Skel_Mesh`))
  (bind _vehicle (`self.Vehicle`))
  (`SceneComponent.SetHiddenInGame` (`self.Dave`) isHidden false)
  (`PrimitiveComponent.SetMaterial` (`self.Vehicle_Skel_Mesh1`) 0 vehicleMat)
  (`/Engine/EditorBlueprintResources/StandardMacros.IsValid` _radar_skel_mesh
    (:`Is Valid`
      (`PrimitiveComponent.SetMaterial` _radar_skel_mesh 0 radarMat))
    (:`Is Not Valid`
      _))
  (`self.K2_SetActorLocation` _returnvalue cameraLoc false false)
  (`SceneComponent.SetVisibility` (`self.Tertiary_Radar_component_group`) isHidden true)
  (`SceneComponent.SetVisibility` (`self.Secondary_Radar_component_group`) isHidden true)
  (`SceneComponent.SetVisibility` (`self.Radar_component_group`) isHidden true)
  (bind _asturntable_pawn (cast `/Game/Blueprints/Turntable/Turntable_Pawn` _returnvalue))
  (`/Game/Blueprints/Turntable/Turntable_Pawn.Set_zoom_limit` _asturntable_pawn isHidden)
  (`/Engine/EditorBlueprintResources/StandardMacros.IsValid` _radar_skel_mesh_2
    (:`Is Valid`
      (`PrimitiveComponent.SetMaterial` _radar_skel_mesh_2 0 secondRadarMat))
    (:`Is Not Valid`
      _))
  (`/Engine/EditorBlueprintResources/StandardMacros.IsValid` _secondary_mesh
    (:`Is Valid`
      (`PrimitiveComponent.SetMaterial` _secondary_mesh 0 secondRadarMat))
    (:`Is Not Valid`
      _))
  (`/Engine/EditorBlueprintResources/StandardMacros.IsValid` _vehicle
    (:`Is Valid`
      (`PrimitiveComponent.SetMaterial` _vehicle 0 vehicleMat))
    (:`Is Not Valid`
      _))
  (if isHidden
    (`KismetSystemLibrary.ExecuteConsoleCommand` "r.PostProcessAAQuality 0" null)
    (else
      (`KismetSystemLibrary.ExecuteConsoleCommand` "r.PostProcessAAQuality 5" null))))

(fn `UnitSetup`
  (bind _splinebp (`self.SplineBP`))
  (`/Engine/EditorBlueprintResources/StandardMacros.IsValid` _splinebp
    (:`Is Valid`
      (bind _outactors (`GameplayStatics.GetAllActorsOfClass` "/Game/Blueprints/Freemode_Pawn.Freemode_Pawn_C"))
      (set `self.PlayBackController` (`|GetArrayItem` _outactors))
      (bind _output_get (set `self.Movement_Speed` (/ (`SplineComponent.GetSplineLength` (`/Game/Blueprints/WayPoint.Spline` _splinebp)) (`self.TimeToCompletePath`))))
      (set `self.DistanceAlongSpline` (* _output_get (`self.TimeToStartPath`) -1.0))
      (set `self.GroundRayList` (`|MakeArray` (`SceneComponent.RelativeLocation` (`self.GroundRay1`)) (`SceneComponent.RelativeLocation` (`self.GroundRay2`)) (`SceneComponent.RelativeLocation` (`self.GroundRay3`)) (`SceneComponent.RelativeLocation` (`self.GroundRay4`)))))))

(fn `UserConstructionScript`
  (bind _radar_skel_mesh (`self.Radar_Skel_Mesh`))
  (bind _radar_skel_mesh_2 (`self.Radar_Skel_Mesh`))
  (bind _returnvalue (`SplineComponent.GetSplineLength` (`/Game/Blueprints/WayPoint.Spline` (`self.SplineBP`))))
  (bind _array (`|MakeArray` (`SceneComponent.RelativeLocation` (`self.MEG`)) (`SceneComponent.RelativeLocation` (`self.ENV`)) (`SceneComponent.RelativeLocation` (`self.PWR`)) (`SceneComponent.RelativeLocation` (`self.ARY`)) (`SceneComponent.RelativeLocation` (`self.GEN`))))
  (bind _returnvalue_2 (/ _returnvalue 100000.0))
  (bind _returnvalue_3 (`KismetMathLibrary.FTrunc` _returnvalue))
  (`/Engine/EditorBlueprintResources/StandardMacros.IsValid` _radar_skel_mesh_2
    (:`Is Valid`
      (`SceneComponent.K2_AttachToComponent` (`self.Radar_component_group`) _radar_skel_mesh_2 (`self.Attach_bone`) "KeepRelative" "KeepWorld" "KeepWorld" true))
    (:`Is Not Valid`
      _))
  (`/Engine/EditorBlueprintResources/StandardMacros.IsValid` _radar_skel_mesh
    (:`Is Valid`
      (`SceneComponent.K2_AttachToComponent` (`self.Secondary_Radar_component_group`) _radar_skel_mesh (`self.Second_Attach_bone`) "KeepRelative" "KeepWorld" "KeepWorld" true))
    (:`Is Not Valid`
      _))
  (for (_array_element _array_index) _array
    (`SceneComponent.K2_SetRelativeLocation` (`|GetArrayItem` (`|MakeArray` (`self.alt_start_point`) (`self.alt_start_point2`) (`self.alt_start_point3`) (`self.alt_start_point4`) (`self.alt_start_point5`)) _array_index) (* _array_element 4.0) false false))
  (set `self.start point origins` _array)
  (if (>= _returnvalue_3 100000)
    (set `self.Spline_length` (`KismetStringLibrary.Concat_StrStr` (`KismetTextLibrary.Conv_TextToString` (`KismetTextLibrary.Conv_DoubleToText` _returnvalue_2 "HalfToEven" false true 1 324 0 2)) " : Km"))
    (elif (>= _returnvalue_3 100)
      (set `self.Spline_length` (`KismetStringLibrary.Concat_StrStr` (`KismetTextLibrary.Conv_TextToString` (`KismetTextLibrary.Conv_DoubleToText` (/ _returnvalue 100.0) "HalfToEven" false true 1 324 0 2)) " : M"))
      (else
        (set `self.Spline_length` (`KismetStringLibrary.Concat_StrStr` (`KismetTextLibrary.Conv_TextToString` (`KismetTextLibrary.Conv_DoubleToText` _returnvalue "HalfToEven" false true 1 324 0 2)) " : Cm")))))
  (set `self.Vehicle_Target_Distance` _returnvalue_2)
  (if (`self.Update Spline Points`)
    (set `self.Update Spline Points` false)
    (`self.StoreSplinePoints`)))