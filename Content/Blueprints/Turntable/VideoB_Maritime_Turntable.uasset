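; Actor Blueprint for the maritime video turntable that puts a media player on screen when play begins.
; BeginPlay creates a Media_player widget, passes its Maritime variable as IsMaritime, and adds the widget to the viewport.
; It then adds a MediaSound component at runtime, with no media player assignment shown in the graph.
; Overlap and Tick events are disabled, and the construction script only calls its parent.
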(event `self.ReceiveBeginPlay`
  (`parent.ReceiveBeginPlay`)
  (bind _returnvalue (`|CreateWidget` "/Game/Blueprints/Turntable/Media_player.Media_player_C" null (`self.Maritime`)))
  (`UserWidget.AddToViewport` _returnvalue 10)
  (`AddComponent|NODE_AddMediaSoundComponent-0`))

(fn `UserConstructionScript`
  (`parent.UserConstructionScript`))