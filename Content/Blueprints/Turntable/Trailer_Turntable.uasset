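; Child vehicle Blueprint for a CEATAC radar rig towing a trailer that follows a spline over terrain.
; Each tick it drives dust particles from speed and colour, then places the trailer behind along the spline using a downward trace.
; Trailer rotation aims at the tow pivot, with up averaged from ground-ray hit normals.
; Parent material events switch default and camo materials; transparent variants are disconnected.
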(event `self.ReceiveBeginPlay`
  (`parent.ReceiveBeginPlay`)
  (if (`self.isTurnTableMode`)
    (`SceneComponent.K2_AddLocalOffset` (`self.Vehicle_Holder`) (0.0 0.0 0.0) false false)))

(event `self.ReceiveTick`
  (params (DeltaSeconds :type "Float (single-precision)"))
  (bind _splinebp (`self.SplineBP`))
  (`parent.ReceiveTick` DeltaSeconds)
  (`ParticleSystemComponent.SetFloatParameter` (`self.ParticleSystem1`) "Speed" (`KismetMathLibrary.MapRangeUnclamped` (`self.Movement_Speed Km/h`) 0.0 25.0 0.0 1.0))
  (`ParticleSystemComponent.SetFloatParameter` (`self.ParticleSystem`) "Speed" (`KismetMathLibrary.MapRangeUnclamped` (`self.Movement_Speed Km/h`) 0.0 25.0 0.0 1.0))
  (`ParticleSystemComponent.SetFloatParameter` (`self.ParticleSystem2`) "Speed" (`KismetMathLibrary.MapRangeUnclamped` (`self.Movement_Speed Km/h`) 0.0 25.0 0.0 1.0))
  (`ParticleSystemComponent.SetFloatParameter` (`self.ParticleSystem3`) "Speed" (`KismetMathLibrary.MapRangeUnclamped` (`self.Movement_Speed Km/h`) 0.0 25.0 0.0 1.0))
  (`ParticleSystemComponent.SetColorParameter` (`self.ParticleSystem`) "Colour" (`self.Dust_colour`))
  (`ParticleSystemComponent.SetColorParameter` (`self.ParticleSystem1`) "Colour" (`self.Dust_colour`))
  (`ParticleSystemComponent.SetColorParameter` (`self.ParticleSystem3`) "Colour" (`self.Dust_colour`))
  (`ParticleSystemComponent.SetColorParameter` (`self.ParticleSystem2`) "Colour" (`self.Dust_colour`))
  (`/Engine/EditorBlueprintResources/StandardMacros.IsValid` _splinebp
    (:`Is Valid`
      (if (< (+ (`self.DistanceAlongSpline`) 561.0) (`SplineComponent.GetSplineLength` (`/Game/Blueprints/WayPoint.Spline` _splinebp)))
        (`self.SetTrailerPos`)
        (`self.SetTrailerRotation`)))))

(event `self.Isolate_radar`
  (bind ((`Base_2_7B6D7139420B2937790D43B314199C77` _base) (`Camo_11_A738607545FDC8CD65B190956D8927DB` _camo) (`BaseTransparent_12_E6EF7356455DBAE5C34D6EAB042D956A` _basetransparent) (`CamoTransparent_13_BF6E64424D7F41DC8F57559C4F365B04` _camotransparent)) (break `/Game/Blueprints/VehicleMaterials` (`self.Trailer_Materials`)))
  (bind ((`Base_2_7B6D7139420B2937790D43B314199C77` _base_2) (`Camo_11_A738607545FDC8CD65B190956D8927DB` _camo_2) (`BaseTransparent_12_E6EF7356455DBAE5C34D6EAB042D956A` _basetransparent_2) (`CamoTransparent_13_BF6E64424D7F41DC8F57559C4F365B04` _camotransparent_2)) (break `/Game/Blueprints/VehicleMaterials` (`self.CEATAC_Materials`)))
  (`parent.Isolate_radar`)
  (if (`self.isTransparent`)
    _
    (else
      _))
  (`PrimitiveComponent.SetMaterial` (`self.CEATAC_Rigged`) 0 (select `/Game/Blueprints/Enums/VehicleMaterialType` (`self.MaterialType`) :`NewEnumerator0` _base_2 :`NewEnumerator1` _camo_2))
  (`PrimitiveComponent.SetMaterial` (`self.trailer_mesh`) 0 (select `/Game/Blueprints/Enums/VehicleMaterialType` (`self.MaterialType`) :`NewEnumerator0` _base :`NewEnumerator1` _camo)))

(event `self.ForceMatChange`
  (params (Type :type "/Game/Blueprints/Enums/VehicleMaterialType Enum" :default "NewEnumerator0"))
  (bind (_base _camo) (break `/Game/Blueprints/VehicleMaterials` (`self.CEATAC_Materials`)))
  (bind (_base_2 _camo_2) (break `/Game/Blueprints/VehicleMaterials` (`self.Trailer_Materials`)))
  (`parent.ForceMatChange` Type)
  (if (`self.isTransparent`) :!label _label
    _
    (else
      _))
  (`PrimitiveComponent.SetMaterial` (`self.CEATAC_Rigged`) 0 (select `/Game/Blueprints/Enums/VehicleMaterialType` (`self.MaterialType`) :`NewEnumerator0` _base :`NewEnumerator1` _camo))
  (`PrimitiveComponent.SetMaterial` (`self.trailer_mesh`) 0 (select `/Game/Blueprints/Enums/VehicleMaterialType` (`self.MaterialType`) :`NewEnumerator0` _base_2 :`NewEnumerator1` _camo_2)))

(event `self.Swap_textures`
  (`parent.Swap_textures`)
  (goto _label))

(fn `CalculateTrailerUp`
  (returns (newNormal :type "Vector Structure"))
  (set `self.TrailerUp` (0.0 0.0 0.0))
  (for _index (range (`KismetArrayLibrary.Array_Length` (`self.TrailerRays`)))
    (bind _returnvalue (`SceneComponent.K2_GetComponentLocation` (`|GetArrayItem` (`self.TrailerRays`) _index)))
    (bind _outhit (`KismetSystemLibrary.LineTraceSingleForObjects` _returnvalue (- _returnvalue (0.0 0.0 1000.0)) (`|MakeArray` "ObjectTypeQuery1" :!type "EObjectTypeQuery Enum")))
    (set `self.TrailerUp` (+ (`self.TrailerUp`) (`.ImpactNormal` (`GameplayStatics.BreakHitResult` _outhit)))))
  (return (`KismetMathLibrary.Normal` (`self.TrailerUp`))))

(fn `SetTrailerPos`
  (bind _returnvalue (`SplineComponent.GetLocationAtDistanceAlongSpline` (`/Game/Blueprints/WayPoint.Spline` (`self.SplineBP`)) (- (`self.DistanceAlongSpline`) 582.0) "World"))
  (bind _outhit (`KismetSystemLibrary.LineTraceSingleForObjects` _returnvalue (- _returnvalue (0.0 0.0 10000.0)) (`|MakeArray` "ObjectTypeQuery1" :!type "EObjectTypeQuery Enum")))
  (`SceneComponent.K2_SetWorldLocation` (`self.trailer_mesh`) (`.Location` (`GameplayStatics.BreakHitResult` _outhit)) false false))

(fn `SetTrailerRotation`
  (bind _splinebp (`self.SplineBP`))
  (bind _returnvalue (`SceneComponent.K2_GetComponentLocation` (`self.Trailer_Pivot`)))
  (bind _returnvalue_2 (`SceneComponent.K2_GetComponentLocation` (`self.trailer_mesh`)))
  (bind _returnvalue_3 (`SplineComponent.GetLocationAtDistanceAlongSpline` (`/Game/Blueprints/WayPoint.Spline` (`self.SplineBP`)) (- (`self.DistanceAlongSpline`) 461.0) "World"))
  (`/Engine/EditorBlueprintResources/StandardMacros.IsValid` _splinebp
    (:`Is Valid`
      (if (< (- (`self.DistanceAlongSpline`) 561.0) (`SplineComponent.GetSplineLength` (`/Game/Blueprints/WayPoint.Spline` _splinebp)))
        (`KismetSystemLibrary.LineTraceSingleForObjects` :`Start` _returnvalue_3 :`End` (- _returnvalue_3 (0.0 0.0 10000.0)) :`ObjectTypes` (`|MakeArray` "ObjectTypeQuery1" :!type "EObjectTypeQuery Enum") :`DrawTime` 0.1)
        (bind _newnormal (`self.CalculateTrailerUp`))
        (`SceneComponent.K2_SetWorldRotation` (`self.trailer_mesh`) (`KismetMathLibrary.FindLookAtRotation` _returnvalue_2 _returnvalue) false false)
        (`SceneComponent.K2_SetWorldRotation` (`self.trailer_mesh`) (`KismetMathLibrary.MakeRotFromXZ` (- _returnvalue _returnvalue_2) _newnormal) false false)))))

(fn `UserConstructionScript`
  (bind _trailergroundray1 (`self.TrailerGroundRay1`))
  (bind _trailergroundray2 (`self.TrailerGroundRay2`))
  (bind _trailergroundray3 (`self.TrailerGroundRay3`))
  (bind _trailergroundray4 (`self.TrailerGroundRay4`))
  (bind _trailergroundray5 (`self.TrailerGroundRay5`))
  (bind _trailergroundray6 (`self.TrailerGroundRay6`))
  (set `self.RadarRef1` (`self.CEATAC_Rigged`))
  (set `self.RadarRef2` (`self.trailer_mesh`))
  (set `self.RadarRef3` (`self.Vehicle_Skel_Mesh1`))
  (`parent.UserConstructionScript`)
  (`BlueprintSetLibrary.Set_RemoveItems` (`|MakeSet` _trailergroundray1 _trailergroundray2 _trailergroundray3 _trailergroundray4 _trailergroundray5 _trailergroundray6) (`self.GroundRaysLeft`))
  (set `self.TrailerRays` (`|MakeArray` _trailergroundray1 _trailergroundray2 _trailergroundray3 _trailergroundray4 _trailergroundray5 _trailergroundray6)))