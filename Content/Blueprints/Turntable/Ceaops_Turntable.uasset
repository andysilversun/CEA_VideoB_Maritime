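; Ceaops turntable radar actor, a child Blueprint that supplies its radar, base and tile child actors to parent logic.
; Construction fills the radar references and two tile arrays, optionally changing letter attach points on two tiles.
; Tick drives dust particle speed and colour from movement speed and dust colour.
; Isolation, forced material changes and texture swaps select default or camo, opaque or transparent materials; isolation also toggles EnvironmentControl visibility.
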(event `self.ReceiveBeginPlay`
  (`parent.ReceiveBeginPlay`))

(event `self.ReceiveTick`
  (params (DeltaSeconds :type "Float (single-precision)"))
  (`parent.ReceiveTick` DeltaSeconds)
  (`ParticleSystemComponent.SetFloatParameter` (`self.ParticleSystem1`) "Speed" (`KismetMathLibrary.MapRangeUnclamped` (`self.Movement_Speed Km/h`) 0.0 25.0 0.0 1.0))
  (`ParticleSystemComponent.SetFloatParameter` (`self.ParticleSystem`) "Speed" (`KismetMathLibrary.MapRangeUnclamped` (`self.Movement_Speed Km/h`) 0.0 25.0 0.0 1.0))
  (`ParticleSystemComponent.SetColorParameter` (`self.ParticleSystem`) "Colour" (`self.Dust_colour`))
  (`ParticleSystemComponent.SetColorParameter` (`self.ParticleSystem1`) "Colour" (`self.Dust_colour`)))

(event `self.Isolate_radar`
  (bind _materialtype (`self.MaterialType`))
  (bind _materialtype_2 (`self.MaterialType`))
  (bind ((`Base_2_7B6D7139420B2937790D43B314199C77` _base) (`Camo_11_A738607545FDC8CD65B190956D8927DB` _camo) (`BaseTransparent_12_E6EF7356455DBAE5C34D6EAB042D956A` _basetransparent) (`CamoTransparent_13_BF6E64424D7F41DC8F57559C4F365B04` _camotransparent)) (break `/Game/Blueprints/VehicleMaterials` (`self.BaseMaterials`)))
  (bind ((`Base_2_7B6D7139420B2937790D43B314199C77` _base_2) (`Camo_11_A738607545FDC8CD65B190956D8927DB` _camo_2) (`BaseTransparent_12_E6EF7356455DBAE5C34D6EAB042D956A` _basetransparent_2) (`CamoTransparent_13_BF6E64424D7F41DC8F57559C4F365B04` _camotransparent_2)) (break `/Game/Blueprints/VehicleMaterials` (`self.RadarMaterials`)))
  (`parent.Isolate_radar`)
  (if (`self.isTransparent`)
    (`PrimitiveComponent.SetMaterial` (`self.Base`) 0 (select `/Game/Blueprints/Enums/VehicleMaterialType` _materialtype_2 :`NewEnumerator0` _basetransparent :`NewEnumerator1` _camotransparent))
    (`PrimitiveComponent.SetMaterial` (`self.Radar`) 0 (select `/Game/Blueprints/Enums/VehicleMaterialType` _materialtype :`NewEnumerator0` _basetransparent_2 :`NewEnumerator1` _camotransparent_2))
    (else
      (`PrimitiveComponent.SetMaterial` (`self.Base`) 0 (select `/Game/Blueprints/Enums/VehicleMaterialType` _materialtype_2 :`NewEnumerator0` _base :`NewEnumerator1` _camo))
      (`PrimitiveComponent.SetMaterial` (`self.Radar`) 0 (select `/Game/Blueprints/Enums/VehicleMaterialType` _materialtype :`NewEnumerator0` _base_2 :`NewEnumerator1` _camo_2))))
  (`SceneComponent.SetVisibility` (`self.Environment_Control`) (`self.isTransparent`) true))

(event `self.ForceMatChange`
  (params (Type :type "/Game/Blueprints/Enums/VehicleMaterialType Enum" :default "NewEnumerator0"))
  (bind (_base _camo) (break `/Game/Blueprints/VehicleMaterials` (`self.BaseMaterials`)))
  (bind ((`BaseTransparent_12_E6EF7356455DBAE5C34D6EAB042D956A` _basetransparent) (`CamoTransparent_13_BF6E64424D7F41DC8F57559C4F365B04` _camotransparent)) (break `/Game/Blueprints/VehicleMaterials` (`self.BaseMaterials`)))
  (bind ((`Base_2_7B6D7139420B2937790D43B314199C77` _base_2) (`Camo_11_A738607545FDC8CD65B190956D8927DB` _camo_2)) (break `/Game/Blueprints/VehicleMaterials` (`self.RadarMaterials`)))
  (bind ((`BaseTransparent_12_E6EF7356455DBAE5C34D6EAB042D956A` _basetransparent_2) (`CamoTransparent_13_BF6E64424D7F41DC8F57559C4F365B04` _camotransparent_2)) (break `/Game/Blueprints/VehicleMaterials` (`self.RadarMaterials`)))
  (`parent.ForceMatChange` Type)
  (if (`self.isTransparent`) :!label _label
    (`PrimitiveComponent.SetMaterial` (`self.Base`) 0 (select `/Game/Blueprints/Enums/VehicleMaterialType` (`self.MaterialType`) :`NewEnumerator0` _basetransparent :`NewEnumerator1` _camotransparent))
    (`PrimitiveComponent.SetMaterial` (`self.Radar`) 0 (select `/Game/Blueprints/Enums/VehicleMaterialType` (`self.MaterialType`) :`NewEnumerator0` _basetransparent_2 :`NewEnumerator1` _camotransparent_2))
    (else
      (`PrimitiveComponent.SetMaterial` (`self.Base`) 0 (select `/Game/Blueprints/Enums/VehicleMaterialType` (`self.MaterialType`) :`NewEnumerator0` _base :`NewEnumerator1` _camo))
      (`PrimitiveComponent.SetMaterial` (`self.Radar`) 0 (select `/Game/Blueprints/Enums/VehicleMaterialType` (`self.MaterialType`) :`NewEnumerator0` _base_2 :`NewEnumerator1` _camo_2)))))

(event `self.Swap_textures`
  (`parent.Swap_textures`)
  (goto _label))

(fn `UserConstructionScript`
  (bind _radar (`self.Radar`))
  (set `self.RadarRef1` _radar)
  (set `self.RadarRef2` _radar)
  (set `self.ArrayList1` (`|MakeArray` (`self.Tile`) (`self.Tile6`)))
  (set `self.ArrayList2` (`|MakeArray` (`self.Tile1`) (`self.Tile2`) (`self.Tile3`) (`self.Tile4`)))
  (`parent.UserConstructionScript`)
  (if (`self.SetLetter`)
    (bind _astile (cast `/Game/Blueprints/Tile` (`ChildActorComponent.ChildActor` (`self.Tile`)))
      (:`then`
        (`/Game/Blueprints/Tile.ChangeLetterAttachPoint` _astile))
      (:`CastFailed`
        _))
    (bind _astile_2 (cast `/Game/Blueprints/Tile` (`ChildActorComponent.ChildActor` (`self.Tile6`))))
    (`/Game/Blueprints/Tile.ChangeLetterAttachPoint` _astile_2)))