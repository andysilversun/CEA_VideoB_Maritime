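; Turntable display Blueprint for the CTES ADVMTTES variant, a child actor presenting a dual-face CTES radar unit and its generator.
; The construction script registers both components as the parent's radar references.
; Overrides of IsolateRadar, ForceMatChange and SwapTextures run parent logic, then reapply generator and CTES materials, choosing opaque or transparent from IsTransparent and default or camo from MaterialType.
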(event `self.Isolate_radar`
  (bind _materialtype (`self.MaterialType`))
  (bind _materialtype_2 (`self.MaterialType`))
  (bind ((`Base_2_7B6D7139420B2937790D43B314199C77` _base) (`Camo_11_A738607545FDC8CD65B190956D8927DB` _camo) (`BaseTransparent_12_E6EF7356455DBAE5C34D6EAB042D956A` _basetransparent) (`CamoTransparent_13_BF6E64424D7F41DC8F57559C4F365B04` _camotransparent)) (break `/Game/Blueprints/VehicleMaterials` (`self.GeneratorMaterials`)))
  (bind ((`Base_2_7B6D7139420B2937790D43B314199C77` _base_2) (`Camo_11_A738607545FDC8CD65B190956D8927DB` _camo_2) (`BaseTransparent_12_E6EF7356455DBAE5C34D6EAB042D956A` _basetransparent_2) (`CamoTransparent_13_BF6E64424D7F41DC8F57559C4F365B04` _camotransparent_2)) (break `/Game/Blueprints/VehicleMaterials` (`self.CTESMaterials`)))
  (bind _returnvalue (select `/Game/Blueprints/Enums/VehicleMaterialType` _materialtype_2 :`NewEnumerator0` _base_2 :`NewEnumerator1` _camo_2))
  (bind _returnvalue_2 (select `/Game/Blueprints/Enums/VehicleMaterialType` _materialtype_2 :`NewEnumerator0` _basetransparent_2 :`NewEnumerator1` _camotransparent_2))
  (`parent.Isolate_radar`)
  (if (`self.isTransparent`)
    (`PrimitiveComponent.SetMaterial` (`self.Generator`) 0 (select `/Game/Blueprints/Enums/VehicleMaterialType` _materialtype :`NewEnumerator0` _basetransparent :`NewEnumerator1` _camotransparent))
    (`PrimitiveComponent.SetMaterial` (`self.CTES_Dual_Face`) 0 _returnvalue_2)
    (`PrimitiveComponent.SetMaterial` (`self.CTES_Dual_Face`) 1 _returnvalue_2)
    (else
      (`PrimitiveComponent.SetMaterial` (`self.Generator`) 0 (select `/Game/Blueprints/Enums/VehicleMaterialType` _materialtype :`NewEnumerator0` _base :`NewEnumerator1` _camo))
      (`PrimitiveComponent.SetMaterial` (`self.CTES_Dual_Face`) 0 _returnvalue)
      (`PrimitiveComponent.SetMaterial` (`self.CTES_Dual_Face`) 1 _returnvalue))))

(event `self.ForceMatChange`
  (params (Type :type "/Game/Blueprints/Enums/VehicleMaterialType Enum" :default "NewEnumerator0"))
  (bind (_base _camo) (break `/Game/Blueprints/VehicleMaterials` (`self.GeneratorMaterials`)))
  (bind ((`BaseTransparent_12_E6EF7356455DBAE5C34D6EAB042D956A` _basetransparent) (`CamoTransparent_13_BF6E64424D7F41DC8F57559C4F365B04` _camotransparent)) (break `/Game/Blueprints/VehicleMaterials` (`self.GeneratorMaterials`)))
  (bind ((`Base_2_7B6D7139420B2937790D43B314199C77` _base_2) (`Camo_11_A738607545FDC8CD65B190956D8927DB` _camo_2)) (break `/Game/Blueprints/VehicleMaterials` (`self.CTESMaterials`)))
  (bind ((`BaseTransparent_12_E6EF7356455DBAE5C34D6EAB042D956A` _basetransparent_2) (`CamoTransparent_13_BF6E64424D7F41DC8F57559C4F365B04` _camotransparent_2)) (break `/Game/Blueprints/VehicleMaterials` (`self.CTESMaterials`)))
  (bind _returnvalue (select `/Game/Blueprints/Enums/VehicleMaterialType` (`self.MaterialType`) :`NewEnumerator0` _base_2 :`NewEnumerator1` _camo_2))
  (bind _returnvalue_2 (select `/Game/Blueprints/Enums/VehicleMaterialType` (`self.MaterialType`) :`NewEnumerator0` _basetransparent_2 :`NewEnumerator1` _camotransparent_2))
  (`parent.ForceMatChange` Type)
  (if (`self.isTransparent`) :!label _label
    (`PrimitiveComponent.SetMaterial` (`self.Generator`) 0 (select `/Game/Blueprints/Enums/VehicleMaterialType` (`self.MaterialType`) :`NewEnumerator0` _basetransparent :`NewEnumerator1` _camotransparent))
    (`PrimitiveComponent.SetMaterial` (`self.CTES_Dual_Face`) 0 _returnvalue_2)
    (`PrimitiveComponent.SetMaterial` (`self.CTES_Dual_Face`) 1 _returnvalue_2)
    (else
      (`PrimitiveComponent.SetMaterial` (`self.Generator`) 0 (select `/Game/Blueprints/Enums/VehicleMaterialType` (`self.MaterialType`) :`NewEnumerator0` _base :`NewEnumerator1` _camo))
      (`PrimitiveComponent.SetMaterial` (`self.CTES_Dual_Face`) 0 _returnvalue)
      (`PrimitiveComponent.SetMaterial` (`self.CTES_Dual_Face`) 1 _returnvalue))))

(event `self.Swap_textures`
  (`parent.Swap_textures`)
  (goto _label))

(fn `UserConstructionScript`
  (set `self.RadarRef1` (`self.CTES_Dual_Face`))
  (set `self.RadarRef2` (`self.Generator`))
  (`parent.UserConstructionScript`))