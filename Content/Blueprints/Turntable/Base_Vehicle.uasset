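; Base radar vehicle actor that either serves as an interactive turntable exhibit or drives along a spline, chosen by whether the player pawn is a Turntable_Pawn.
; Turntable mode adds auto-rotation, animation UI, exploded component zoom and a transparent-material radar isolation view.
; Spline mode sets position by distance, ground-tracing Land and Water types and tilting Land to averaged ray normals.
; Construction attaches radar groups to bones and configures child Tile arrays.
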(event `self.ReceiveBeginPlay`
  (bind _asturntable_pawn (cast `/Game/Blueprints/Turntable/Turntable_Pawn` (`GameplayStatics.GetPlayerPawn` 0))
    (:`then`
      (set `self.pawn` _asturntable_pawn)
      (`self.TurntableSetup`))
    (:`CastFailed`
      (set `self.isTurnTableMode` false)
      (`SceneComponent.SetVisibility` (`self.Dave`) false false)
      (`/Engine/EditorBlueprintResources/StandardMacros.IsValid` (`self.SplineBP`)
        (:`Is Valid`
          (`self.SetPosition`)
          (`self.SetRotation`))
        (:`Is Not Valid`
          _))))
  (`|ExecutionSequence`
    (:`then_0`
      (if (`self.UseCamoMaterials`)
        (`self.ForceMatChange` "NewEnumerator1")))
    (:`then_1`
      (set `self.isTransparent` true)
      (`/Game/Blueprints/Turntable/Turntable_Object_Iface.Isolate_radar`)
      (`KismetSystemLibrary.Delay` 0.2)
      (bind _returnvalue (`|SpawnActorFromClass` (`self.Stats`) (`KismetMathLibrary.MakeTransform` (0.0 0.0 0.0)) "Undefined" "OverrideRootScale" null null))
      (set `self.StatsRef` _returnvalue)
      (`KismetSystemLibrary.Delay` 0.1)
      (`self.UnitSetup`))))

(event `self.ReceiveTick`
  (params (DeltaSeconds :type "Float (single-precision)"))
  (if (`self.isTurnTableMode`)
    (if (`self.isAutoRotate`)
      (`SceneComponent.K2_AddLocalRotation` (`self.Vehicle_Skel_Mesh1`) (* (struct :`Yaw` 1.0) (* DeltaSeconds (`self.RotateSpeed`))) false false))
    (else
      (`self.Movement`)
      (if (!= (`self.EnableTileUpdates`) (`self.EnableTileUpdates_Prev`))
        (`self.ToggleTileUpdates`)))))

(event `change_zoom`
  (params (Alpha :type "Float (double-precision)"))
  ;[1 1 1] Zooming
  (for (_array_element _array_index) (`|MakeArray` (`self.MEG`) (`self.ENV`) (`self.PWR`) (`self.ARY`) (`self.GEN`))
    (`/Engine/EditorBlueprintResources/StandardMacros.IsValid` _array_element
      (:`Is Valid`
        (`SceneComponent.K2_SetRelativeLocation` _array_element (`KismetMathLibrary.VLerp` (`|GetArrayItem` (`self.start point origins`) _array_index) (`SceneComponent.RelativeLocation` (`|GetArrayItem` (`|MakeArray` (`self.alt_start_point`) (`self.alt_start_point2`) (`self.alt_start_point3`) (`self.alt_start_point4`) (`self.alt_start_point5`)) _array_index)) Alpha) false false)))))

(event `/Game/Blueprints/Turntable/Turntable_Object_Iface.Rotate`
  (params (Automated :type Boolean) (Speed :type "Float (single-precision)") (Custom_Angle :type "Float (single-precision)"))
  ;[1 1 1] Turntable rotation
  (set `self.isAutoRotate` Automated)
  (set `self.RotateSpeed` (`KismetMathLibrary.FClamp` (+ (`self.RotateSpeed`) Speed) -360.0 360.0)))

(event `/Game/Blueprints/Turntable/Turntable_Object_Iface.Isolate_radar`
  (bind ((`Base_2_7B6D7139420B2937790D43B314199C77` _base) (`Camo_11_A738607545FDC8CD65B190956D8927DB` _camo) (`BaseTransparent_12_E6EF7356455DBAE5C34D6EAB042D956A` _basetransparent) (`CamoTransparent_13_BF6E64424D7F41DC8F57559C4F365B04` _camotransparent)) (break `/Game/Blueprints/VehicleMaterials` (`self.BaseVehicleMats`)))
  ;[1 1 1] Show radar components
  (bind _output_get (set `self.isTransparent` (not (`self.isTransparent`))))
  (if _output_get
    (`self.ToggleIsolation` (`self.Vehicle_Skel_Mesh1`) (select `/Game/Blueprints/Enums/VehicleMaterialType` (`self.MaterialType`) :`NewEnumerator0` _basetransparent :`NewEnumerator1` _camotransparent) (`SceneComponent.K2_GetComponentLocation` (`self.Radar_Cam`)) true)
    (`SceneComponent.SetHiddenInGame` (`self.BlockOutBoxes2`) true false)
    (`SceneComponent.SetHiddenInGame` (`self.BlockOutBoxes1`) true false)
    (`SceneComponent.SetHiddenInGame` (`self.BlockOutBoxes3`) true false)
    (else
      (`self.ToggleIsolation` (`self.Vehicle_Skel_Mesh1`) (select `/Game/Blueprints/Enums/VehicleMaterialType` (`self.MaterialType`) :`NewEnumerator0` _base :`NewEnumerator1` _camo) (`SceneComponent.K2_GetComponentLocation` (`self.Main_Cam`)))
      (`SceneComponent.SetHiddenInGame` (`self.BlockOutBoxes3`) false false)
      (`SceneComponent.SetHiddenInGame` (`self.BlockOutBoxes2`) false false)
      (`SceneComponent.SetHiddenInGame` (`self.BlockOutBoxes1`) false false)))
  (if (`self.isTurnTableMode`)
    (`SceneComponent.SetHiddenInGame` (`self.Dave`) (`self.isTransparent`) false)))

(event `ForceMatChange`
  (params (Type :type "/Game/Blueprints/Enums/VehicleMaterialType Enum" :default "NewEnumerator0"))
  (bind (_base _camo) (break `/Game/Blueprints/VehicleMaterials` (`self.BaseVehicleMats`)))
  (bind ((`BaseTransparent_12_E6EF7356455DBAE5C34D6EAB042D956A` _basetransparent) (`CamoTransparent_13_BF6E64424D7F41DC8F57559C4F365B04` _camotransparent)) (break `/Game/Blueprints/VehicleMaterials` (`self.BaseVehicleMats`)))
  ;[1 1 1] Change texture
  (set `self.MaterialType` Type)
  (if (`self.isTransparent`) :!label _label
    (`PrimitiveComponent.SetMaterial` (`self.Vehicle_Skel_Mesh1`) 0 (select `/Game/Blueprints/Enums/VehicleMaterialType` (`self.MaterialType`) :`NewEnumerator0` _basetransparent :`NewEnumerator1` _camotransparent))
    (else
      (`PrimitiveComponent.SetMaterial` (`self.Vehicle_Skel_Mesh1`) 0 (select `/Game/Blueprints/Enums/VehicleMaterialType` (`self.MaterialType`) :`NewEnumerator0` _base :`NewEnumerator1` _camo)))))

(event `Kill`
  (bind _statsref (`self.StatsRef`))
  ;[1 1 1] Destroy Vehicle
  (`/Engine/EditorBlueprintResources/StandardMacros.IsValid` _statsref
    (:`Is Valid`
      (`self.K2_DestroyActor` _statsref)
      (`KismetSystemLibrary.Delay` 0.1))
    (:`Is Not Valid`
      _))
  (`self.K2_DestroyActor`))

(event `/Game/Blueprints/Turntable/Turntable_Object_Iface.Swap_textures`
  ;[1 1 1] Change texture
  (`self.SwapMaterial`)
  (goto _label))

(event `ToggleTileUpdates`
  (for _array_element (`self.ArrayList1`)
    (bind _astile (cast `/Game/Blueprints/Tile` (`ChildActorComponent.ChildActor` _array_element)))
    (set `/Game/Blueprints/Tile.Update` (`self.EnableTileUpdates`) _astile))
  (for _array_element_2 (`self.ArrayList2`)
    (bind _astile_2 (cast `/Game/Blueprints/Tile` (`ChildActorComponent.ChildActor` _array_element_2)))
    (set `/Game/Blueprints/Tile.Update` (`self.EnableTileUpdates`) _astile_2))
  (set `self.EnableTileUpdates_Prev` (`self.EnableTileUpdates`)))

(event `/Game/Blueprints/Turntable/Turntable_Object_Iface.Play/Pause Anim`
  (bind _anim_ui (`self.anim_ui`))
  (bind _radarref1 (`self.RadarRef1`))
  (bind _returnvalue (`SkeletalMeshComponent.GetAnimInstance` _radarref1))
  ;[1 1 1] Play/Pause Animations
  (`/Engine/EditorBlueprintResources/StandardMacros.IsValid` _radarref1
    (:`Is Valid`
      (if (`self.Multi_mode`)
        (message `/Game/Blueprints/Turntable/Anim_IF.Set_play_mode` _returnvalue _anim_ui)
        (else
          (`/Engine/EditorBlueprintResources/StandardMacros.FlipFlop`
            (:`A`
              (message `/Game/Blueprints/Turntable/Anim_IF.Set_Play_rate` _returnvalue -1.0 _anim_ui))
            (:`B`
              (message `/Game/Blueprints/Turntable/Anim_IF.Set_Play_rate` _returnvalue 1.0 _anim_ui))))))))

(event `deploy/stow stands`
  (params (forward :type Boolean))
  (bind _radarref1 (`self.RadarRef1`))
  ;[1 1 1] Deply/Sow Stands
  (`/Engine/EditorBlueprintResources/StandardMacros.IsValid` _radarref1
    (:`Is Valid`
      (if forward
        (`SkeletalMeshComponent.SetPlayRate` _radarref1 1.0)
        (else
          (`SkeletalMeshComponent.SetPlayRate` _radarref1 -1.0)))
      (`SkeletalMeshComponent.Play` _radarref1 false))))

(fn `CalculateNewUp`
  (returns (newNormal :type "Vector Structure"))
  (set `self.NewUpDir` (0.0 0.0 0.0))
  (for _index (range (`KismetArrayLibrary.Array_Length` (`self.GroundRayList`)))
    (bind _returnvalue (`SceneComponent.K2_GetComponentLocation` (`|GetArrayItem` (`self.GroundRayList`) _index)))
    (bind _outhit (`KismetSystemLibrary.LineTraceSingleForObjects` _returnvalue (- _returnvalue (0.0 0.0 1000.0)) (`|MakeArray` "ObjectTypeQuery1" :!type "EObjectTypeQuery Enum")))
    (set `self.NewUpDir` (+ (`self.NewUpDir`) (`.ImpactNormal` (`GameplayStatics.BreakHitResult` _outhit)))))
  (return (`KismetMathLibrary.Normal` (`self.NewUpDir`))))

(fn `LandSeaRotation`
  (bind _vehicle_front (`self.vehicle_front`))
  (bind (_returnvalue_roll _returnvalue_pitch _returnvalue_yaw) (`KismetMathLibrary.BreakRotator` (`SceneComponent.K2_GetComponentRotation` _vehicle_front)))
  (bind _relativelocation_x (`KismetMathLibrary.BreakVector` (`SceneComponent.RelativeLocation` _vehicle_front)))
  (bind _returnvalue (`SplineComponent.GetLocationAtDistanceAlongSpline` (`/Game/Blueprints/WayPoint.Spline` (`self.SplineBP`)) (+ (`self.DistanceAlongSpline`) 100.0) "World"))
  (bind (_returnvalue_roll_2 _returnvalue_pitch_2 _returnvalue_yaw_2) (`KismetMathLibrary.BreakRotator` (`SplineComponent.GetRotationAtDistanceAlongSpline` (`/Game/Blueprints/WayPoint.Spline` (`self.SplineBP`)) (+ (+ _relativelocation_x (`self.DistanceAlongSpline`)) 50.0) "World")))
  (bind _outhit (`KismetSystemLibrary.LineTraceSingleForObjects` :`Start` _returnvalue :`End` (- _returnvalue (0.0 0.0 10000.0)) :`ObjectTypes` (`|MakeArray` "ObjectTypeQuery1" :!type "EObjectTypeQuery Enum") :`DrawTime` 0.1))
  (switch `/Game/Blueprints/Enums/VehicleType` (`self.VehicleType`)
    (:`NewEnumerator0`
      ;[1 1 1] Land Rotation
      (bind _newnormal (`self.CalculateNewUp`))
      (bind _returnvalue_2 (`KismetMathLibrary.Normal` (- (`.ImpactPoint` (`GameplayStatics.BreakHitResult` _outhit)) (`SceneComponent.K2_GetComponentLocation` (`self.DefaultSceneRoot`)))))
      (`SceneComponent.K2_SetWorldRotation` (`self.DefaultSceneRoot`) (`KismetMathLibrary.MakeRotFromZX` _newnormal _returnvalue_2) false false)
      (set `self.Turn_Rotation` (`KismetMathLibrary.MakeRotator` 0.0 0.0 (- _returnvalue_yaw_2 _returnvalue_yaw))))
    (:`NewEnumerator1`
      ;[1 1 1] Boat Rotation
      (`SceneComponent.K2_SetWorldRotation` (`self.DefaultSceneRoot`) (`KismetMathLibrary.Conv_VectorToRotator` _returnvalue_2) false false))))

(fn `Movement`
  (bind (_turn_rotation_roll _turn_rotation_pitch _turn_rotation_yaw) (`KismetMathLibrary.BreakRotator` (`self.Turn_Rotation`)))
  (bind _returnvalue (* (`self.Movement_Speed Km/h`) 36.0))
  (`/Engine/EditorBlueprintResources/StandardMacros.IsValid` (`self.SplineBP`)
    (:`Is Valid`
      (set `self.DistanceAlongSpline` (+ (* (`GameplayStatics.GetWorldDeltaSeconds`) _returnvalue) (`self.DistanceAlongSpline`)))
      (`self.SetPosition`)
      (`self.SetRotation`)
      (set `self.LastLocation` (`SceneComponent.K2_GetComponentLocation` (`self.DefaultSceneRoot`)))
      (message `/Game/Blueprints/Wheel_Anim_IF.UPDATE` (`SkeletalMeshComponent.GetAnimInstance` (`self.Vehicle_Skel_Mesh1`)) _returnvalue (`KismetMathLibrary.MapRangeClamped` _turn_rotation_yaw -45.0 45.0 -1.0 1.0)))))

(fn `SetPosition`
  (bind _returnvalue (`SplineComponent.GetLocationAtDistanceAlongSpline` (`/Game/Blueprints/WayPoint.Spline` (`self.SplineBP`)) (`self.DistanceAlongSpline`) "World"))
  (switch `/Game/Blueprints/Enums/VehicleType` (`self.VehicleType`)
    (:`NewEnumerator0`
      (bind _outhit (`KismetSystemLibrary.LineTraceSingleForObjects` _returnvalue (- _returnvalue (0.0 0.0 10000.0)) (`|MakeArray` "ObjectTypeQuery1" :!type "EObjectTypeQuery Enum") :!label _label))
      (`SceneComponent.K2_SetWorldLocation` (`self.DefaultSceneRoot`) (`.Location` (`GameplayStatics.BreakHitResult` _outhit)) false false))
    (:`NewEnumerator1`
      (goto _label))
    (:`NewEnumerator2`
      (`SceneComponent.K2_SetWorldLocation` (`self.DefaultSceneRoot`) _returnvalue false false :!label _label_2))
    (:`NewEnumerator3`
      (goto _label_2))))

(fn `SetRotation`
  (bind _splinebp (`self.SplineBP`))
  (`/Engine/EditorBlueprintResources/StandardMacros.IsValid` _splinebp
    (:`Is Valid`
      (if (< (`self.DistanceAlongSpline`) (`SplineComponent.GetSplineLength` (`/Game/Blueprints/WayPoint.Spline` _splinebp)))
        (switch `/Game/Blueprints/Enums/VehicleType` (`self.VehicleType`)
          (:`NewEnumerator0`
            _)
          (:`NewEnumerator1`
            _))
        (`self.LandSeaRotation`)))))

(fn `StoreSplinePoints`
  (bind _pointinfo (`self.PointInfo`))
  (bind _spline (`/Game/Blueprints/WayPoint.Spline` (`self.SplineBP`)))
  (for _index (range (`SplineComponent.GetNumberOfSplinePoints` _spline))
    (if (< _index (`KismetArrayLibrary.Array_Length` _pointinfo))
      (if (`|EnumEquality` (`.Action_11_86D8DEFF4DFBE2E260EC2AA4693510AD` (break `/Game/Blueprints/SplineStruct` (`|GetArrayItem` _pointinfo _index))) "NewEnumerator3")
        (`KismetArrayLibrary.Array_Add` _pointinfo (make `/Game/Blueprints/SplineStruct` _index (`SplineComponent.GetDistanceAlongSplineAtSplinePoint` _spline _index) "NewEnumerator3") :!label _label))
      (else
        (goto _label)))))

(fn `SwapMaterial`
  (switch `/Game/Blueprints/Enums/VehicleMaterialType` (`self.MaterialType`)
    (:`NewEnumerator0`
      (set `self.MaterialType` "NewEnumerator1"))
    (:`NewEnumerator1`
      (set `self.MaterialType` "NewEnumerator0"))))

(fn `ToggleIsolation`
  (params (SkeletalMesh :type "SkeletalMeshComponent Object Reference") (material :type "MaterialInstance Object Reference") (cameraLoc :type "Vector Structure") (isHidden :type Boolean))
  (bind _returnvalue (`GameplayStatics.GetPlayerPawn` 0))
  (`/Engine/EditorBlueprintResources/StandardMacros.IsValid` SkeletalMesh
    (:`Is Valid`
      (`PrimitiveComponent.SetMaterial` SkeletalMesh 0 material)
      (if (`self.isTurnTableMode`)
        (`self.K2_SetActorLocation` _returnvalue cameraLoc false false)
        (`SceneComponent.SetVisibility` (`self.BlockOutBoxes1`) isHidden true)
        (`SceneComponent.SetVisibility` (`self.BlockOutBoxes2`) isHidden true)
        (`SceneComponent.SetVisibility` (`self.BlockOutBoxes3`) isHidden true)
        (bind _asturntable_pawn (cast `/Game/Blueprints/Turntable/Turntable_Pawn` _returnvalue))
        (`/Game/Blueprints/Turntable/Turntable_Pawn.Set_zoom_limit` _asturntable_pawn isHidden)
        (if isHidden
          (`KismetSystemLibrary.ExecuteConsoleCommand` "r.PostProcessAAQuality 0" null)
          (else
            (`KismetSystemLibrary.ExecuteConsoleCommand` "r.PostProcessAAQuality 5" null)))))))

(fn `TurntableSetup`
  (bind _pawn (`self.pawn`))
  (bind _anim_ui (`self.anim_ui`))
  (`self.change_zoom` (`KismetMathLibrary.MapRangeClamped` (`/Game/Blueprints/Turntable/Turntable_Pawn.Spring arm length` _pawn) 200.0 1300.0 0.0 1.0))
  (`/Game/Blueprints/Turntable/Turntable_Pawn.hide idle` _pawn)
  (`/Game/Blueprints/Turntable/Turntable_Pawn.drag screen messege` _pawn)
  (bind _foundwidgets (`WidgetBlueprintLibrary.GetAllWidgetsOfClass` "/Game/Blueprints/Turntable/TurnTable_Anim_UI.TurnTable_Anim_UI_C" false))
  (bind _output (`|GetArrayItem` _foundwidgets))
  (`/Engine/EditorBlueprintResources/StandardMacros.IsValid` _output
    (:`Is Valid`
      (set `self.anim_ui` _output))
    (:`Is Not Valid`
      (bind _returnvalue (`|CreateWidget` "/Game/Blueprints/Turntable/TurnTable_Anim_UI.TurnTable_Anim_UI_C"))
      (set `self.anim_ui` _returnvalue)
      (`UserWidget.AddToViewport` _anim_ui 1)))
  (message `/Game/Blueprints/Turntable/Anim_IF.setup anim` (`SkeletalMeshComponent.GetAnimInstance` (`self.RadarRef1`)) _anim_ui)
  (`self.K2_SetActorLocation` (`GameplayStatics.GetPlayerPawn` 0) (`SceneComponent.K2_GetComponentLocation` (`self.Main_Cam`)) false false))

(fn `UnitSetup`
  (bind (_relativelocation_x _relativelocation_y _relativelocation_z) (`KismetMathLibrary.BreakVector` (`SceneComponent.RelativeLocation` (`self.GroundRay4`))))
  (bind _relativelocation_x_2 (`KismetMathLibrary.BreakVector` (`SceneComponent.RelativeLocation` (`self.GroundRay3`))))
  (bind _relativelocation_x_3 (`KismetMathLibrary.BreakVector` (`SceneComponent.RelativeLocation` (`self.GroundRay1`))))
  (bind (_relativelocation_x_4 _relativelocation_y_2 _relativelocation_z_2) (`KismetMathLibrary.BreakVector` (`SceneComponent.RelativeLocation` (`self.GroundRay3`))))
  (for _index (range 1 (`self.NumberOfGroundCheckRays`))
    (bind _returnvalue (* _index (/ (- _relativelocation_x_2 _relativelocation_x_3) (`KismetMathLibrary.Conv_IntToDouble` (`self.NumberOfGroundCheckRays`)))))
    (`AddComponent|NODE_AddArrowComponent-0` :`RelativeTransform` (`KismetMathLibrary.MakeTransform` (`KismetMathLibrary.MakeVector` _returnvalue _relativelocation_y_2 _relativelocation_z_2)))
    (`AddComponent|NODE_AddArrowComponent-1` :`RelativeTransform` (`KismetMathLibrary.MakeTransform` (`KismetMathLibrary.MakeVector` _returnvalue _relativelocation_y _relativelocation_z))))
  (set `self.GroundRayList` (`self.K2_GetComponentsByClass` "/Script/Engine.ArrowComponent")))

(fn `UserConstructionScript`
  (bind _radarref1 (`self.RadarRef1`))
  (bind _radarref3 (`self.RadarRef3`))
  (bind _radarref2 (`self.RadarRef2`))
  (bind _returnvalue (`SplineComponent.GetSplineLength` (`/Game/Blueprints/WayPoint.Spline` (`self.SplineBP`))))
  (bind _array (`|MakeArray` (`SceneComponent.RelativeLocation` (`self.MEG`)) (`SceneComponent.RelativeLocation` (`self.ENV`)) (`SceneComponent.RelativeLocation` (`self.PWR`)) (`SceneComponent.RelativeLocation` (`self.ARY`)) (`SceneComponent.RelativeLocation` (`self.GEN`))))
  (bind _returnvalue_2 (/ _returnvalue 100000.0))
  (bind _returnvalue_3 (`KismetMathLibrary.FTrunc` _returnvalue))
  (`|ExecutionSequence`
    (:`then_0`
      (`/Engine/EditorBlueprintResources/StandardMacros.IsValid` _radarref1
        (:`Is Valid`
          (`SceneComponent.K2_AttachToComponent` (`self.Radar_Component_Group1`) _radarref1 (`self.Attach_bone`) "KeepRelative" "KeepWorld" "KeepWorld" true))
        (:`Is Not Valid`
          _))
      (for (_array_element _array_index) _array
        (`SceneComponent.K2_SetRelativeLocation` (`|GetArrayItem` (`|MakeArray` (`self.alt_start_point`) (`self.alt_start_point2`) (`self.alt_start_point3`) (`self.alt_start_point4`) (`self.alt_start_point5`)) _array_index) (* _array_element 4.0) false false))
      (set `self.start point origins` _array)
      (if (>= _returnvalue_3 100000)
        (set `self.Spline_length` (`KismetStringLibrary.Concat_StrStr` (`KismetTextLibrary.Conv_TextToString` (`KismetTextLibrary.Conv_DoubleToText` _returnvalue_2 "HalfToEven" false true 1 324 0 2)) " : Km"))
        (elif (>= _returnvalue_3 100)
          (set `self.Spline_length` (`KismetStringLibrary.Concat_StrStr` (`KismetTextLibrary.Conv_TextToString` (`KismetTextLibrary.Conv_DoubleToText` (/ _returnvalue 100.0) "HalfToEven" false true 1 324 0 2)) " : M"))
          (else
            (set `self.Spline_length` (`KismetStringLibrary.Concat_StrStr` (`KismetTextLibrary.Conv_TextToString` (`KismetTextLibrary.Conv_DoubleToText` _returnvalue "HalfToEven" false true 1 324 0 2)) " : Cm")))))
      (set `self.Vehicle_Target_Distance` _returnvalue_2)
      (`|ExecutionSequence`
        (:`then_0`
          (if (`self.Update Spline Points`)
            (set `self.Update Spline Points` false)
            (`self.StoreSplinePoints`))
          (`SceneComponent.SetVisibility` (`self.BlockOutBoxes1`) false true)
          (`SceneComponent.SetVisibility` (`self.BlockOutBoxes2`) false true)
          (`SceneComponent.SetVisibility` (`self.BlockOutBoxes3`) false true)
          (if (`|EnumInequality` (`self.TileArrayType`) "NewEnumerator3")
            (if (`self.DisplayMainRadars`)
              (for _array_element_2 (`self.ArrayList1`)
                (bind _astile (cast `/Game/Blueprints/Tile` (`ChildActorComponent.ChildActor` _array_element_2)))
                (`/Game/Blueprints/Tile.SetupFromVehicle` _astile (`self.TileArrayType`) (`self.ShowBands`)))
              (for _array_element_3 (`self.ArrayList2`)
                (bind _astile_2 (cast `/Game/Blueprints/Tile` (`ChildActorComponent.ChildActor` _array_element_3)))
                (`/Game/Blueprints/Tile.SetupFromVehicle` _astile_2 "NewEnumerator3" false)
                (`SceneComponent.SetVisibility` _array_element_3 true false))
              (elif (`self.DisplaySubRadars`)
                (for _array_element_4 (`self.ArrayList2`)
                  (bind _astile_3 (cast `/Game/Blueprints/Tile` (`ChildActorComponent.ChildActor` _array_element_4)))
                  (`/Game/Blueprints/Tile.SetupFromVehicle` _astile_3 (`self.TileArrayType`) (`self.ShowBands`))
                  (`SceneComponent.SetVisibility` _array_element_4 true false))
                (for _array_element_5 (`self.ArrayList1`)
                  (bind _astile_4 (cast `/Game/Blueprints/Tile` (`ChildActorComponent.ChildActor` _array_element_5)))
                  (`/Game/Blueprints/Tile.SetupFromVehicle` _astile_4 "NewEnumerator3" false))
                (else
                  (for _array_element_6 (`self.GetAllChildActors` true)
                    (bind _astile_5 (cast `/Game/Blueprints/Tile` _array_element_6))
                    (`/Game/Blueprints/Tile.SetupFromVehicle` _astile_5 (`self.TileArrayType`) (`self.ShowBands`))
                    (`SceneComponent.SetVisibility` (`Actor.RootComponent` _array_element_6) true false)))))
            (else
              (`SceneComponent.SetVisibility` (`self.Radar_Component_Group1`) false true)
              (`SceneComponent.SetVisibility` (`self.Radar_Component_Group2`) false true)
              (`SceneComponent.SetVisibility` (`self.Radar_Component_Group3`) false true)
              (for _array_element_7 (`self.GetAllChildActors` true)
                (`SceneComponent.SetVisibility` (`Actor.RootComponent` _array_element_7) false true)))))
        (:`then_1`
          (`/Engine/EditorBlueprintResources/StandardMacros.IsValid` (`self.SplineBP`)
            (:`Is Valid`
              (`self.SetPosition`)
              (`self.SetRotation`))))))
    (:`then_1`
      (`/Engine/EditorBlueprintResources/StandardMacros.IsValid` _radarref2
        (:`Is Valid`
          (`SceneComponent.K2_AttachToComponent` (`self.Radar_Component_Group2`) _radarref2 (`self.Second_Attach_bone`) "KeepRelative" "KeepWorld" "KeepWorld" true))))
    (:`then_2`
      (`/Engine/EditorBlueprintResources/StandardMacros.IsValid` _radarref3
        (:`Is Valid`
          (`SceneComponent.K2_AttachToComponent` (`self.Radar_Component_Group3`) _radarref3 (`self.Third_Attach_bone`) "KeepRelative" "KeepWorld" "KeepWorld" true))))))