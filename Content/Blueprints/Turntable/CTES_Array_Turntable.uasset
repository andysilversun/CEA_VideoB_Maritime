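; CTES_Array_Turntable is a child turntable Blueprint that displays a CTES unit on a single generator base with switchable materials.
; The construction script assigns both components to the parent's radar reference slots before calling the parent's construction logic.
; IsolateRadar, ForceMatChange and SwapTextures call their parent versions, then set both components to default or camo materials, opaque or transparent according to IsTransparent.
; ForceMatChange and SwapTextures share the material logic, which IsolateRadar duplicates.
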(event `self.ReceiveBeginPlay`
  (`parent.ReceiveBeginPlay`))

(event `self.Isolate_radar`
  (bind _materialtype (`self.MaterialType`))
  (bind _materialtype_2 (`self.MaterialType`))
  (bind ((`Base_2_7B6D7139420B2937790D43B314199C77` _base) (`Camo_11_A738607545FDC8CD65B190956D8927DB` _camo) (`BaseTransparent_12_E6EF7356455DBAE5C34D6EAB042D956A` _basetransparent) (`CamoTransparent_13_BF6E64424D7F41DC8F57559C4F365B04` _camotransparent)) (break `/Game/Blueprints/VehicleMaterials` (`self.BaseVehicleMats`)))
  (bind ((`Base_2_7B6D7139420B2937790D43B314199C77` _base_2) (`Camo_11_A738607545FDC8CD65B190956D8927DB` _camo_2) (`BaseTransparent_12_E6EF7356455DBAE5C34D6EAB042D956A` _basetransparent_2) (`CamoTransparent_13_BF6E64424D7F41DC8F57559C4F365B04` _camotransparent_2)) (break `/Game/Blueprints/VehicleMaterials` (`self.GeneratorMaterials`)))
  (`parent.Isolate_radar`)
  (if (`self.isTransparent`)
    (`PrimitiveComponent.SetMaterial` (`self.Single_Generator_Base`) 0 (select `/Game/Blueprints/Enums/VehicleMaterialType` _materialtype :`NewEnumerator0` _basetransparent :`NewEnumerator1` _camotransparent))
    (`PrimitiveComponent.SetMaterial` (`self.CTES`) 0 (select `/Game/Blueprints/Enums/VehicleMaterialType` _materialtype_2 :`NewEnumerator0` _basetransparent_2 :`NewEnumerator1` _camotransparent_2))
    (else
      (`PrimitiveComponent.SetMaterial` (`self.Single_Generator_Base`) 0 (select `/Game/Blueprints/Enums/VehicleMaterialType` _materialtype :`NewEnumerator0` _base :`NewEnumerator1` _camo))
      (`PrimitiveComponent.SetMaterial` (`self.CTES`) 0 (select `/Game/Blueprints/Enums/VehicleMaterialType` _materialtype_2 :`NewEnumerator0` _base_2 :`NewEnumerator1` _camo_2)))))

(event `self.ForceMatChange`
  (params (Type :type "/Game/Blueprints/Enums/VehicleMaterialType Enum" :default "NewEnumerator0"))
  (bind (_base _camo) (break `/Game/Blueprints/VehicleMaterials` (`self.BaseVehicleMats`)))
  (bind ((`BaseTransparent_12_E6EF7356455DBAE5C34D6EAB042D956A` _basetransparent) (`CamoTransparent_13_BF6E64424D7F41DC8F57559C4F365B04` _camotransparent)) (break `/Game/Blueprints/VehicleMaterials` (`self.BaseVehicleMats`)))
  (bind ((`Base_2_7B6D7139420B2937790D43B314199C77` _base_2) (`Camo_11_A738607545FDC8CD65B190956D8927DB` _camo_2)) (break `/Game/Blueprints/VehicleMaterials` (`self.GeneratorMaterials`)))
  (bind ((`BaseTransparent_12_E6EF7356455DBAE5C34D6EAB042D956A` _basetransparent_2) (`CamoTransparent_13_BF6E64424D7F41DC8F57559C4F365B04` _camotransparent_2)) (break `/Game/Blueprints/VehicleMaterials` (`self.GeneratorMaterials`)))
  (`parent.ForceMatChange` Type)
  (if (`self.isTransparent`) :!label _label
    (`PrimitiveComponent.SetMaterial` (`self.Single_Generator_Base`) 0 (select `/Game/Blueprints/Enums/VehicleMaterialType` (`self.MaterialType`) :`NewEnumerator0` _basetransparent :`NewEnumerator1` _camotransparent))
    (`PrimitiveComponent.SetMaterial` (`self.CTES`) 0 (select `/Game/Blueprints/Enums/VehicleMaterialType` (`self.MaterialType`) :`NewEnumerator0` _basetransparent_2 :`NewEnumerator1` _camotransparent_2))
    (else
      (`PrimitiveComponent.SetMaterial` (`self.Single_Generator_Base`) 0 (select `/Game/Blueprints/Enums/VehicleMaterialType` (`self.MaterialType`) :`NewEnumerator0` _base :`NewEnumerator1` _camo))
      (`PrimitiveComponent.SetMaterial` (`self.CTES`) 0 (select `/Game/Blueprints/Enums/VehicleMaterialType` (`self.MaterialType`) :`NewEnumerator0` _base_2 :`NewEnumerator1` _camo_2)))))

(event `self.Swap_textures`
  (`parent.Swap_textures`)
  (goto _label))

(fn `UserConstructionScript`
  (bind _ctes (`self.CTES`))
  (set `self.RadarRef1` _ctes)
  (set `self.RadarRef2` _ctes)
  (set `self.RadarRef3` (`self.Single_Generator_Base`))
  (`parent.UserConstructionScript`))