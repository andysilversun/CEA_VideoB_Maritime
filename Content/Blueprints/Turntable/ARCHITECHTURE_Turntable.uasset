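; Turntable actor Blueprint that sets up the media player UI and its sound component when play begins.
; It reads MODE from the first Turntable_system_controler in the level and passes it to a new Media_player widget as a land or maritime flag.
; The widget is added to the viewport and a MediaSound component is attached to the actor, with no other active logic.
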(event `self.ReceiveBeginPlay`
  (`parent.ReceiveBeginPlay`)
  (bind _outactors (`GameplayStatics.GetAllActorsOfClass` "/Game/Blueprints/Turntable/Turntable_system_controler.Turntable_system_controler_C"))
  (bind _returnvalue (`|CreateWidget` "/Game/Blueprints/Turntable/Media_player.Media_player_C" null (select `/Game/Blueprints/Enums/TurntableType` (`/Game/Blueprints/Turntable/Turntable_system_controler.MODE` (`|GetArrayItem` _outactors)) :`NewEnumerator1` true)))
  (`UserWidget.AddToViewport` _returnvalue 10)
  (`AddComponent|NODE_AddMediaSoundComponent-0`))

(fn `UserConstructionScript`
  (`parent.UserConstructionScript`))