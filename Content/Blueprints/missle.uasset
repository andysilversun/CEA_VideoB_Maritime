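; Homing missile actor that launches after a delay or on fire, flies at Target and detonates at close range.
; Tick feeds two gates: one moves it forward, the other opens after LockOnDelay and lerps rotation toward Target, tightening as it nears.
; A one-shot detonation spawns an explosion if CanKillTarget, stops the trail and calls SelfDetonate on a missile Target.
; Movement is per-frame without delta time; the destroy logic is unconnected.
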(event `self.ReceiveBeginPlay`
  (bind _target (`self.target`))
  (`KismetSystemLibrary.Delay` (`self.delay`))
  (`ActorComponent.Activate` (`self.ParticleSystem`) false :!label _label)
  (`KismetSystemLibrary.Delay` 1.0)
  (`|ExecutionSequence`
    (:`then_0`
      (goto _label_3 :!via `Open`))
    (:`then_1`
      (`KismetSystemLibrary.Delay` (`self.Lock On Delay`))
      (goto _label_4 :!via `Open`))))

(event `fire`
  (goto _label))

(event `Self detonate`
  (bind _target (`self.target`))
  (set `self.can kill_target` false)
  (`/Engine/EditorBlueprintResources/StandardMacros.DoOnce` false :!label _label_2
    (:`Completed`
      (if (`self.can kill_target`)
        (`GameplayStatics.SpawnEmitterAtLocation` "/Game/_CEARepositoryFiles/Particles/Missile/missle_detonation.missle_detonation" (`self.K2_GetActorLocation` _target) (struct) (5.0 5.0 5.0)))
      (`SceneComponent.SetHiddenInGame` (`self.Cylinder`) false false)
      (`ActorComponent.Deactivate` (`self.ParticleSystem`))
      (bind _asmissle (cast `/Game/Blueprints/missle` _target))
      (`self.Self detonate` _asmissle)
      (goto _label_3 :!via `Close`))))

(event `self.ReceiveTick`
  (params (DeltaSeconds :type "Float (single-precision)"))
  (`/Engine/EditorBlueprintResources/StandardMacros.Gate` true :!label _label_3
    (:`Exit`
      (`self.K2_AddActorLocalOffset` (`KismetMathLibrary.MakeVector` (`KismetMathLibrary.MapRangeUnclamped` (`self.Speed`) 0.0 1.0 0.0 3000.0)))
      (`/Engine/EditorBlueprintResources/StandardMacros.Gate` true :!label _label_4
        (:`Exit`
          (`self.K2_SetActorRotation` (`KismetMathLibrary.RLerp` (`self.K2_GetActorRotation`) (`KismetMathLibrary.FindLookAtRotation` (`self.K2_GetActorLocation`) (`self.K2_GetActorLocation` (`self.target`))) (`self.Lock_on_strength`) true))
          (if (< (`self.GetDistanceTo` (`self.target`)) 3000.0)
            (set `self.Lock_on_strength` 0.6)
            (if (< (`self.GetDistanceTo` (`self.target`)) 600.0)
              (goto _label_2))))))))

(fn `UserConstructionScript`)