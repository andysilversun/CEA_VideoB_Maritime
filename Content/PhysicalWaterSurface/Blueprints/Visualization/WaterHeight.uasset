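; Demo actor that finds and visualizes the height of the deformed water surface at its fixed X,Y location.
; Construction caches the first WaterSettings actor and the actor's location.
; Each tick, CalculateDeltaOnly samples at that X,Y offset by the previous frame's negated horizontal delta, iteratively compensating for sideways wave displacement.
; A debug sphere is drawn at the fixed X,Y, with Z as sea level plus the height delta.
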(event `self.ReceiveTick`
  (params (DeltaSeconds :type "Float (single-precision)"))
  (bind (_initiallocation_global__x _initiallocation_global__y) (`KismetMathLibrary.BreakVector` (`self.InitialLocation(global)`)))
  (bind (_initiallocation_global__x_2 _initiallocation_global__y_2) (`KismetMathLibrary.BreakVector` (`self.InitialLocation(global)`)))
  ;[1 1 1] This is a demonstration how to calculate the water height at a given location (X,Y)
  (bind _delta (`/Game/PhysicalWaterSurface/Blueprints/WaterSettings.CalculateDeltaOnly` (`self.WaterSettings`) (+ (`self.DeltaPrev`) (`KismetMathLibrary.MakeVector2D` _initiallocation_global__x _initiallocation_global__y)))) ; calculate delta for current frame
  ;;[1 1 1] save for next frame
  (set `self.DeltaPrev` (`KismetMathLibrary.MakeVector2D` (* (.x _delta) -1.0) (* (.y _delta) -1.0)))
  ;;[1 1 1] x and y are fixed
  (`KismetSystemLibrary.DrawDebugSphere` (`KismetMathLibrary.MakeVector` _initiallocation_global__x_2 _initiallocation_global__y_2 (+ (.z _delta) (`/Game/PhysicalWaterSurface/Blueprints/WaterSettings.SeaLevel` (`self.WaterSettings`)))) 5.0 12 (struct :`R` 1.0 :`B` 0.128267 :`A` 1.0)))

(fn `UserConstructionScript`
  (`|ExecutionSequence`
    (:`then_0`
      ;[1 1 1] get reference to WaterSettings
      (bind _outactors (`GameplayStatics.GetAllActorsOfClass` "/Game/PhysicalWaterSurface/Blueprints/WaterSettings.WaterSettings_C"))
      (set `self.WaterSettings` (`KismetArrayLibrary.Array_Get` _outactors)))
    (:`then_1`
      ;[1 1 1] initial location
      (set `self.InitialLocation(global)` (`self.K2_GetActorLocation`)))))