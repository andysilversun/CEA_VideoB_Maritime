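; Debug visualization actor that shows water surface height and its vertical speed at the actor's initial XY location.
; Each tick it queries WaterSettings, feeding back the previous negated horizontal displacement to sample the height above that fixed point.
; Once a tick counter reaches its threshold, it updates velocity and stores the height for the next calculation.
; A debug sphere marks the surface at sea level plus height, with a vertical arrow showing velocity.
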(event EventTick
  (params (DeltaSeconds :type Float%20%28single-precision%29))
  (bind _initiallocation_global_ (Variables|Default|GetInitialLocation%28global%29))
  (bind _tickcount (Variables|Default|GetTickCount))
  (bind _initiallocation_global__2 (Variables|Default|GetInitialLocation%28global%29))
  (Variables|Default|SetDeltaSec DeltaSeconds)
  (Utilities|FlowControl|Sequence
    (:then_0
      ;[1 1 1] calculate current water height
      (bind _delta (Default|CalculateDeltaOnly (Variables|Default|GetWaterSettings) (+ (Variables|Default|GetDeltaPrev) (Math|Vector2D|MakeVector2D (.x _initiallocation_global_) (.y _initiallocation_global_)))))
      (Variables|Default|SetDeltaPrev (Math|Vector2D|MakeVector2D (* (.x _delta) -1.0) (* (.y _delta) -1.0)))
      (Variables|Default|SetHeight (.z _delta)))
    (:then_1
      ;[1 1 1] calculate velocity
      ;;[1 1 1] check if we update on this tick
      (Math|Integer|IncrementInt _tickcount
        (:%20%20
          (if (>= _tickcount (Variables|Default|GetUpdateEveryTick))
            (Utilities|FlowControl|Sequence
              (:then_0
                (Variables|Default|SetVelocity (|((10*({22405A65-43D9-A202-D1DC-8CB7414E70EB}-{08FC4645-4BCD-06B5-903B-DE930B36943E}))/{DB84F7FC-4896-E872-8BB5-6AB0348FEAA4}))))
              (:then_1
                ;;[1 1 1] save height for next tick
                (Variables|Default|SetHeightPrevious (Variables|Default|GetHeight))))))))
    (:then_2
      ;[1 1 1] draw debug sphere and arrow
      (Rendering|Debug|DrawDebugSphere (Math|Vector|MakeVector (.x _initiallocation_global__2) (.y _initiallocation_global__2) (+ (Variables|Default|GetHeight) (Variables|/Game/PhysicalWaterSurface/Blueprints/WaterSettings.WaterSettings_C|GetSeaLevel (Variables|Default|GetWaterSettings)))) 5.0 12 "(R=1.000000,G=0.000000,B=0.128000,A=1.000000)" 0.0)
      (Rendering|Debug|DrawDebugArrow (Math|Vector|MakeVector (.x _initiallocation_global__2) (.y _initiallocation_global__2) (+ (Variables|Default|GetHeight) (Variables|/Game/PhysicalWaterSurface/Blueprints/WaterSettings.WaterSettings_C|GetSeaLevel (Variables|Default|GetWaterSettings)))) (+ (Math|Vector|MakeVector (.x _initiallocation_global__2) (.y _initiallocation_global__2) (+ (Variables|Default|GetHeight) (Variables|/Game/PhysicalWaterSurface/Blueprints/WaterSettings.WaterSettings_C|GetSeaLevel (Variables|Default|GetWaterSettings)))) (Math|Vector|MakeVector 0.0 0.0 (Variables|Default|GetVelocity))) 1e+02 "(R=1.000000,G=0.000000,B=0.128000,A=1.000000)" 0.0))))

(fn ConstructionScript
  (Utilities|FlowControl|Sequence
    (:then_0
      ;[1 1 1] get reference to WaterSettings
      (bind _outactors (Actor|GetAllActorsOfClass "/Game/PhysicalWaterSurface/Blueprints/WaterSettings.WaterSettings_C"))
      (Variables|Default|SetWaterSettings (Utilities|Array|Get(acopy) _outactors)))
    (:then_1
      ;[1 1 1] initial location
      (Variables|Default|SetInitialLocation%28global%29 (Transformation|GetActorLocation)))))