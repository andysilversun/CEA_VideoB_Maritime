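; Demonstration actor that visualizes how a point on the Gerstner-wave water surface moves away from its rest position.
; The construction script caches the first WaterSettings actor in the level and stores the actor's own location as the initial point.
; Each tick it queries CalculateDeltaOnly at that point and draws a red debug sphere at the displaced XY, with height taken from sea level plus the Z delta.
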(event `self.ReceiveTick`
  (params (DeltaSeconds :type "Float (single-precision)"))
  (bind (_initiallocation_global__x _initiallocation_global__y) (`KismetMathLibrary.BreakVector` (`self.InitialLocation(global)`)))
  ;[1 1 1] This is a demonstration how to query the Delta vector, given the initial location.
  ; CalculateDeltaOnly evaluates the Gerstner equations and returns the Delta vector.
  (bind _delta (`/Game/PhysicalWaterSurface/Blueprints/WaterSettings.CalculateDeltaOnly` (`self.WaterSettings`) (`KismetMathLibrary.MakeVector2D` _initiallocation_global__x _initiallocation_global__y)))
  (bind (_returnvalue_x _returnvalue_y) (`KismetMathLibrary.BreakVector` (+ _delta (`self.InitialLocation(global)`))))
  (`KismetSystemLibrary.DrawDebugSphere` (`KismetMathLibrary.MakeVector` _returnvalue_x _returnvalue_y (+ (.z _delta) (`/Game/PhysicalWaterSurface/Blueprints/WaterSettings.SeaLevel` (`self.WaterSettings`)))) 5.0 12 (struct :`R` 1.0 :`B` 0.128267 :`A` 1.0)))

(fn `UserConstructionScript`
  (`|ExecutionSequence`
    (:`then_0`
      ;[1 1 1] get reference to WaterSettings
      (bind _outactors (`GameplayStatics.GetAllActorsOfClass` "/Game/PhysicalWaterSurface/Blueprints/WaterSettings.WaterSettings_C"))
      (set `self.WaterSettings` (`KismetArrayLibrary.Array_Get` _outactors)))
    (:`then_1`
      ;[1 1 1] initial location
      (set `self.InitialLocation(global)` (`self.K2_GetActorLocation`)))))